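; BP_ForgeLevel is a setup Blueprint for the forge level that initializes local multiplayer and the HUD.
; On BeginPlay it creates local players with pawns for controllers 1 to 3, then has the first BP_CameraSystem in the world set the controllers' view.
; It then adds W_HUD to the viewport and hands it the first BP_ServingBench found.
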(event EventBeginPlay
  (Class|GameplayStatics|CreatePlayer 1)
  (Class|GameplayStatics|CreatePlayer 2)
  (Class|GameplayStatics|CreatePlayer 3)
  (bind _outactors (Actor|GetAllActorsOfClass "/Game/Blueprints/Mechanics/BP_CameraSystem.BP_CameraSystem_C"))
  (Default|SetControllersView (Utilities|Array|Get(acopy) _outactors))
  (bind _returnvalue (UserInterface|CreateWidget "/Game/UI/Ordering/W_HUD.W_HUD_C"))
  (UserInterface|Viewport|AddtoViewport _returnvalue 0)
  (bind _outactors_2 (Actor|GetAllActorsOfClass "/Game/Blueprints/LevelBlueprints/BP_ServingBench.BP_ServingBench_C"))
  (Variables|/Game/UI/Ordering/W_HUD.W_HUD_C|SetServingBench _returnvalue (Utilities|Array|Get(acopy) _outactors_2)))

(event EventTick
  (params (DeltaSeconds :type Float%20%28single-precision%29)))

(fn ConstructionScript)