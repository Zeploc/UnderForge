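; MenuController is the menu player controller that lets local players join or leave and start the game.
; It caches the GM_MenuGameMode on BeginPlay and forwards input to it.
; Keyboard and gamepad keys pass this controller's ID to AddPlayer or RemovePlayer, while the Menu action calls StartGame.
; A leftover PlayerToggle call is disconnected and never runs.
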(event EventBeginPlay
  (bind _asgm_menu_game_mode (Utilities|Casting|CastToGM_MenuGameMode (Game|GetGameMode)))
  (Variables|Default|SetGameModeRef _asgm_menu_game_mode))

(event EventTick
  (params (DeltaSeconds :type Float%20%28single-precision%29)))

(event Input|ActionEvents|InputActionMenu
  (params (Key :type Key%20Structure)))

(event Input|ActionEvents|InputActionMenu
  (params (Key :type Key%20Structure))
  (:Pressed
    (Default|StartGame (Variables|Default|GetGameModeRef))))

(event Input|KeyboardEvents|L
  (params (Key :type Key%20Structure))
  (:Pressed
    (bind _returnvalue (Class|GameplayStatics|GetPlayerControllerID self))
    (Default|RemovePlayer (Variables|Default|GetGameModeRef) _returnvalue)))

(event Input|KeyboardEvents|Enter
  (params (Key :type Key%20Structure))
  (:Pressed
    (bind _returnvalue (Class|GameplayStatics|GetPlayerControllerID self))
    (Default|AddPlayer (Variables|Default|GetGameModeRef) _returnvalue)))

(event Input|GamepadEvents|GamepadFaceButtonBottom
  (params (Key :type Key%20Structure))
  (:Pressed
    (bind _returnvalue (Class|GameplayStatics|GetPlayerControllerID self))
    (Default|AddPlayer (Variables|Default|GetGameModeRef) _returnvalue)))

(event Input|GamepadEvents|GamepadFaceButtonRight
  (params (Key :type Key%20Structure))
  (:Pressed
    (bind _returnvalue (Class|GameplayStatics|GetPlayerControllerID self))
    (Default|RemovePlayer (Variables|Default|GetGameModeRef) _returnvalue)))

(fn ConstructionScript)