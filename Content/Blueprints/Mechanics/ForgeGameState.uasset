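; Game state for the forge level that holds the active weapon orders and mirrors the day and wave timers.
; The server adds random orders from the game singleton's weapon list up to the game mode's limit, multicasting additions and completions to each local ForgeControllerBP.
; ProcessItem matches a delivered weapon to an order, reports its durability ratio to GM_ForgeLevel and destroys it.
; Joining clients request a wave timer update from the server.
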(event Custom|MULTI_NewOrder
  (params (Weapon :type EWeapon%20Enum :default "W_NONE") (ID :type Integer%20%28by%20ref%29))
  (bind _returnvalue (Game|GetPlayerController 0))
  (if (Pawn|IsLocalPlayerController _returnvalue)
    (bind _asforge_controller_bp (Utilities|Casting|CastToForgeControllerBP _returnvalue))
    (Default|NewOrder _asforge_controller_bp Weapon ID)
    (Development|PrintString (Utilities|String|Append "New Order " (Utilities|String|ToString(Integer) ID)) true true "(R=1.000000,G=0.731737,B=0.237019,A=1.000000)" 1e+01)))

(event Custom|MULTI_CompleteOrder
  (params (OrderID :type Integer))
  (bind _returnvalue (Game|GetPlayerController 0))
  (if (Pawn|IsLocalPlayerController _returnvalue)
    (bind _asforge_controller_bp (Utilities|Casting|CastToForgeControllerBP _returnvalue))
    (Default|CompleteOrder _asforge_controller_bp OrderID)))

(event Custom|S_SendOutOrders
  (Networking|SwitchHasAuthority
    (:Authority
      (bind _keys (Utilities|Map|Keys (Variables|Default|GetOrders)))
      (for _array_element _keys
        (CallFunction|MULTINewOrder (.Value (Utilities|Map|Find (Variables|Default|GetOrders) _array_element)) _array_element)))))

(event Custom|MULTI_TEST
  (Development|PrintString "Hello"))

(event Custom|MULTI_StartWaveTimer
  (params (Time :type Float%20%28single-precision%29))
  (bind _returnvalue (Utilities|Time|SetTimerbyEvent (delegate Custom|ClearTimer) Time))
  (Variables|Default|SetWaveTimer _returnvalue))

(event Custom|ClearTimer
  (Utilities|Time|ClearandInvalidateTimerbyHandle (Variables|Default|GetWaveTimer)))

(event Custom|GetUpdateWaveTimer
  (bind _asforge_controller_bp (Utilities|Casting|CastToForgeControllerBP (Game|GetPlayerController 0)))
  (Default|SERVERUpdateWaveTimer _asforge_controller_bp))

(event EventBeginPlay
  (Networking|SwitchHasAuthority
    (:Authority
      _)
    (:Remote
      (CallFunction|GetUpdateWaveTimer)))
  (Utilities|FlowControl|Delay 3.0)
  (Networking|SwitchHasAuthority
    (:Authority
      (CallFunction|MULTITEST))))

(event EventTick
  (params (DeltaSeconds :type Float%20%28single-precision%29))
  (bind _forgegm (CallFunction|GetGamemode))
  (Networking|SwitchHasAuthority
    (:Authority
      (Utilities|IsValid _forgegm
        (:Is%20Valid
          (Variables|Default|SetDayTimeRemaining (Utilities|Time|GetTimerRemainingTimebyHandle (Variables|/Game/Blueprints/Mechanics/GM_ForgeLevel.GM_ForgeLevel_C|GetDayTimerHandle _forgegm))))))))

(fn ConstructionScript)

(fn RemoveAllOrders
  (Utilities|Map|Clear (Variables|Default|GetOrders)))

(fn AddBeginningOrders
  (bind _forgegm (CallFunction|GetGamemode))
  (CallFunction|RemoveAllOrders)
  (Utilities|IsValid _forgegm
    (:Is%20Valid
      (for _index (range 1 (Variables|/Game/Blueprints/Mechanics/GM_ForgeLevel.GM_ForgeLevel_C|GetDayNumberOfOrders _forgegm))
        (CallFunction|AddRandomOrder)))))

(fn AddRandomOrder
  (bind _weapons (CallFunction|GetAvailableWeapons))
  (bind _orders (Variables|Default|GetOrders))
  (bind _returnvalue (Utilities|Map|Length _orders))
  (if (< _returnvalue (Variables|/Game/Blueprints/Mechanics/GM_ForgeLevel.GM_ForgeLevel_C|GetMaxOrdersAtATime (CallFunction|GetGamemode)))
    (LocalVariables|SetNewID _returnvalue)
    (bind _output_get (LocalVariables|SetNewOrder (Utilities|Array|Get(acopy) _weapons (Math|Random|RandomInteger (Utilities|Array|Length _weapons)))))
    (Utilities|Map|Add (Variables|Default|GetOrders) (LocalVariables|GetNewID) _output_get)
    (CallFunction|MULTINewOrder (LocalVariables|GetNewOrder) (LocalVariables|GetNewID))))

(fn GetGamemode
  (Utilities|IsValid (Variables|Default|GetForgeGM)
    (:Is%20Valid
      _)
    (:Is%20Not%20Valid
      (bind _asgm_forge_level (Utilities|Casting|CastToGM_ForgeLevel (Game|GetGameMode)))
      (Variables|Default|SetForgeGM _asgm_forge_level)))
  (return (Variables|Default|GetForgeGM)))

(fn CompleteOrder
  (params (OrderID :type Integer))
  (Utilities|Map|Remove (Variables|Default|GetOrders) OrderID)
  (CallFunction|MULTICompleteOrder OrderID))

(fn ProcessItem
  (params (Sword :type Sword%20Item%20Object%20Reference))
  (bind _forgegm (CallFunction|GetGamemode))
  (Networking|SwitchHasAuthority
    (:Authority
      (bind _keys (Utilities|Map|Keys (Variables|Default|GetOrders)))
      (for _array_element _keys
        (if (Utilities|Enum|Equal(Enum) (Variables|/Script/UnderForge.SwordItem|GetWeaponType Sword) (.Value (Utilities|Map|Find (Variables|Default|GetOrders) _array_element)))
          (Utilities|IsValid _forgegm
            (:Is%20Valid
              (bind _asbp_sword (Utilities|Casting|CastToBP_Sword Sword)
                (:then
                  (LocalVariables|SetDurability (/ (Math|Conversions|ToFloat(Integer) (Variables|/Game/Blueprints/ItemsBlueprints/BP_Sword.BP_Sword_C|GetDurability _asbp_sword)) (Math|Conversions|ToFloat(Integer) (Variables|/Game/Blueprints/ItemsBlueprints/BP_Sword.BP_Sword_C|GetMaxDurability _asbp_sword)))))
                (:CastFailed
                  _))
              (Default|CompleteOrder _forgegm _array_element (LocalVariables|GetDurability)))
            (:Is%20Not%20Valid
              _))
          (bind _asbp_forge_player (Utilities|Casting|CastToBP_ForgePlayer (Variables|/Script/UnderForge.PickUpItem|GetHeldPlayer Sword))
            (:then
              (Default|Drop _asbp_forge_player))
            (:CastFailed
              _))
          (Actor|DestroyActor Sword)
          (return))))))

(fn GetCurrentWaveTime
  (bind _wavetimer (Variables|Default|GetWaveTimer))
  (if (Utilities|Time|IsValidTimerHandle _wavetimer)
    (return (+ (Class|KismetSystemLibrary|GetTimerElapsedTimeHandle _wavetimer) (Utilities|Time|GetTimerRemainingTimebyHandle _wavetimer)))
    (else
      (return 0.0))))

(fn GetAvailableWeapons
  (bind (_isvalid _returnvalue) (Class|CommonFunctions|GetGameSingleton))
  (if _isvalid
    (bind _keys (Utilities|Map|Keys (Variables|/Script/UnderForge.UnderForgeSingleton|GetWeapons _returnvalue)))
    (return _keys)))