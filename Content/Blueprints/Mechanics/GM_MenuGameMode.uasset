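; Game mode for the main menu and local multiplayer ready screen, supporting up to four players.
; BeginPlay shows the menu, plays music and pre-creates three extra local players.
; A bool array tracks who has joined and updates the ready widget; removing an unjoined player returns to the menu if nobody is ready.
; StartGame saves the array to ForgeGameInstance, removes unused players and opens MainLevel.
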(event EventBeginPlay
  (bind _returnvalue (Game|GetPlayerController 0))
  (bind _returnvalue_2 (UserInterface|CreateWidget "/Game/UI/MainMenu/W_MainMenu.W_MainMenu_C" _returnvalue))
  (UserInterface|Viewport|AddtoViewport _returnvalue_2 0)
  (Variables|Default|SetMenuScreenWidget _returnvalue_2)
  (Variables|/Script/Engine.PlayerController|SetbShowMouseCursor _returnvalue true)
  (Input|SetInputModeGameandUI _returnvalue (Variables|/Game/UI/MainMenu/W_MainMenu.W_MainMenu_C|GetPlayButton _returnvalue_2) "DoNotLock" true)
  (Audio|PlaySound2D (Variables|Default|GetMenuMusic))
  (for _index (range 1 3)
    (Class|GameplayStatics|CreatePlayer _index)))

(event EventTick
  (params (DeltaSeconds :type Float%20%28single-precision%29)))

(fn ConstructionScript)

(fn AddPlayer
  (params (PlayerControllerID :type Integer))
  (bind _readyscreenwidget (Variables|Default|GetReadyScreenWidget))
  (Utilities|Array|SetArrayElem (Variables|Default|GetArrayOfBools) PlayerControllerID true)
  (Utilities|IsValid _readyscreenwidget
    (:Is%20Valid
      (Default|SetPlayerText _readyscreenwidget PlayerControllerID true))))

(fn RemovePlayer
  (params (PlayerControllerID :type Integer))
  (bind _arrayofbools (Variables|Default|GetArrayOfBools))
  (bind _readyscreenwidget (Variables|Default|GetReadyScreenWidget))
  (if (Utilities|Array|Get(acopy) _arrayofbools PlayerControllerID)
    (Utilities|Array|SetArrayElem _arrayofbools PlayerControllerID false)
    (Utilities|IsValid _readyscreenwidget
      (:Is%20Valid
        (Default|SetPlayerText _readyscreenwidget PlayerControllerID false)))
    (else
      (CallFunction|ChecktoGoBack))))

(fn PlayerToggle
  (params (PlayerControllerID :type Integer))
  (if (Utilities|Array|Get(acopy) (Variables|Default|GetArrayOfBools) PlayerControllerID)
    (CallFunction|RemovePlayer PlayerControllerID)
    (else
      (CallFunction|AddPlayer PlayerControllerID))))

(fn DisplayPlayerScreen
  (Utilities|IsValid (Variables|Default|GetReadyScreenWidget)
    (:Is%20Valid
      (Widget|SetVisibility (Variables|Default|GetReadyScreenWidget) "Visible"))
    (:Is%20Not%20Valid
      (bind _returnvalue (UserInterface|CreateWidget "/Game/UI/MainMenu/Ready.Ready_C" (Game|GetPlayerController 0)))
      (bind _output_get (Variables|Default|SetReadyScreenWidget _returnvalue))
      (UserInterface|Viewport|AddtoViewport _output_get 0))))

(fn DisplayMenuScreen
  (Utilities|IsValid (Variables|Default|GetMenuScreenWidget)
    (:Is%20Valid
      (Widget|SetVisibility (Variables|Default|GetMenuScreenWidget) "Visible"))
    (:Is%20Not%20Valid
      (bind _returnvalue (UserInterface|CreateWidget "/Game/UI/MainMenu/W_MainMenu.W_MainMenu_C" (Game|GetPlayerController 0)))
      (bind _output_get (Variables|Default|SetMenuScreenWidget _returnvalue))
      (UserInterface|Viewport|AddtoViewport _output_get 0))))

(fn HidePlayerScreen
  (bind _readyscreenwidget (Variables|Default|GetReadyScreenWidget))
  (Utilities|IsValid _readyscreenwidget
    (:Is%20Valid
      (Widget|SetVisibility _readyscreenwidget "Hidden"))))

(fn HideMenuScreen
  (bind _menuscreenwidget (Variables|Default|GetMenuScreenWidget))
  (Utilities|IsValid _menuscreenwidget
    (:Is%20Valid
      (Widget|SetVisibility _menuscreenwidget "Hidden"))))

(fn ChecktoGoBack
  (bind _array_element (Utilities|Array|ForEachLoopwithBreak (Variables|Default|GetArrayOfBools) :!label _label)
    (:LoopBody
      (if _array_element
        (LocalVariables|SetAllPlayersUnready false)
        (goto _label Break)))
    (:Completed
      (if (LocalVariables|GetAllPlayersUnready)
        (CallFunction|DisplayMenuScreen)
        (CallFunction|HidePlayerScreen)))))

(fn StartGame
  (bind _hasplayer (CallFunction|HasPlayer))
  (if _hasplayer
    (bind _asforge_game_instance (Utilities|Casting|CastToForgeGameInstance (Game|GetGameInstance)))
    (Variables|/Game/Blueprints/Mechanics/ForgeGameInstance.ForgeGameInstance_C|SetPlayerState _asforge_game_instance (Variables|Default|GetArrayOfBools))
    (CallFunction|RemoveAllUnusedPlayerControllers)
    (Game|OpenLevel(byName) "MainLevel")))

(fn HasPlayer
  (bind _array_element (Utilities|Array|ForEachLoopwithBreak (Variables|Default|GetArrayOfBools))
    (:LoopBody
      (if _array_element
        (return true)))
    (:Completed
      (return false))))

(fn RemoveAllUnusedPlayerControllers
  (for _index (range 1 3)
    (if (not (Utilities|Array|Get(acopy) (Variables|Default|GetArrayOfBools) _index))
      (Class|GameplayStatics|RemovePlayer (Game|GetPlayerController _index) true))))