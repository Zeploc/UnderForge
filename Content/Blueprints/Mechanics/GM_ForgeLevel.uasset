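; Game mode for the forge level, running a local co-op order-fulfilment game for up to four players in escalating days.
; BeginPlay syncs local players and controller IDs with the game instance, then wires up camera, HUD, serving bench and smeltery.
; Named timers feed orders to the HUD and end each day, starting a longer, busier one or Game Over if orders remain.
; It also handles currency, pausing, end-screen stats and restart cleanup.
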(event EventBeginPlay
  (bind _asforge_game_instance (Utilities|Casting|CastToForgeGameInstance (Game|GetGameInstance)))
  (Variables|Default|SetGameInstanceRef _asforge_game_instance)
  (CallFunction|AddandRemovePlayers) ; Runs first, gets array of controllers
  (bind _outactors (Actor|GetAllActorsOfClass "/Game/Blueprints/Mechanics/BP_CameraSystem.BP_CameraSystem_C"))
  (bind _output_get (Variables|Default|SetCameraControllerRef (Utilities|Array|Get(acopy) _outactors)))
  (Default|SetControllersView _output_get)
  (bind _returnvalue (UserInterface|CreateWidget "/Game/UI/Ordering/W_HUD.W_HUD_C"))
  (bind _output_get_2 (Variables|UIWidgets|SetHUDRef _returnvalue))
  (UserInterface|Viewport|AddtoViewport _output_get_2 0)
  (bind _outactors_2 (Actor|GetAllActorsOfClass "/Game/Blueprints/LevelBlueprints/BP_ServingBench.BP_ServingBench_C"))
  (Variables|/Game/UI/Ordering/W_HUD.W_HUD_C|SetServingBench _returnvalue (Utilities|Array|Get(acopy) _outactors_2))
  (CallFunction|RestartGame)
  (bind _returnvalue_2 (UserInterface|CreateWidget "/Game/UI/Screens/W_PauseScreen.W_PauseScreen_C"))
  (bind _output_get_3 (Variables|UIWidgets|SetPauseScreen _returnvalue_2))
  (UserInterface|Viewport|AddtoViewport _output_get_3 0)
  (Widget|SetVisibility _output_get_3 "Hidden")
  (bind _outactors_3 (Actor|GetAllActorsOfClass "/Game/Blueprints/LevelBlueprints/BP_Smeltery.BP_Smeltery_C"))
  (Default|SetReferences (Utilities|Array|Get(acopy) _outactors_3)))

(event EventTick
  (params (DeltaSeconds :type Float%20%28single-precision%29)))

(fn ConstructionScript)

(fn AddCurrency
  (params (Gained :type Float%20%28single-precision%29))
  (Audio|PlaySound2D 0) ; Play Coin/Money sound
  (bind _output_get (Variables|Game|SetCurrency (+ Gained (Variables|Game|GetCurrency))))
  (Variables|HudUI|SetStringCurrency (Utilities|String|ToString(Integer) (Math|Float|Round _output_get)))
  (Math|Integer|IncrementInt (Variables|Stats|GetTotalOrdersCompleted)))

(fn NewDay
  (bind _currentday (Variables|DayCycle|GetCurrentDay))
  (if (== (Variables|DayCycle|GetCurrentDay) 0) ; If starting Game
    _
    (else
      (Variables|DayOrders|SetDayNumberOfOrders (+ (Variables|DayOrders|GetDayNumberOfOrders) (Variables|DayOrders|GetOrderIncreaseRate)))
      (Variables|DayCycle|SetDayTime (+ (Variables|DayCycle|GetDayTime) (Variables|DayCycle|GetDayTimeIncreaseRate)))
      (Variables|DayOrders|SetOrdersSent 0)
      (Variables|DayOrders|SetCurrentOrderDelay (/ (* (Variables|DayCycle|GetDayTime) 6e+01) (Math|Conversions|ToFloat(Integer) (Variables|DayOrders|GetDayNumberOfOrders))))))
  (Math|Integer|IncrementInt _currentday
    (:%20%20
      (Variables|HudUI|SetCurrentDayString (Utilities|String|Append "Day " (Utilities|String|ToString(Integer) _currentday)))
      (bind _returnvalue (Utilities|Time|SetTimerbyFunctionName 0 "EndDay" (* (Variables|DayCycle|GetDayTime) 6e+01)))
      (Variables|DayCycle|SetDayTimerHandle _returnvalue)
      (CallFunction|AddOrder))))

(fn EndDay
  (Utilities|Time|ClearandInvalidateTimerbyHandle (Variables|DayCycle|GetDayTimerHandle))
  (bind _remainingorders (Default|GetRemainingOrders (Variables|UIWidgets|GetHUDRef)))
  (if (> _remainingorders 0) ; True if orders are remaining
    (CallFunction|GameOver)
    (else
      (CallFunction|NewDay))))

(fn GameOver
  (Game|SetGamePaused true)
  (CallFunction|DisplayEndScreen true)
  (Default|SetEndStats (Variables|UIWidgets|GetEnd%20Screen) 4 (Variables|DayCycle|GetCurrentDay) (Variables|Stats|GetTotalOrdersCompleted) (Variables|Default|GetTotalPartsCreated) (Math|Float|Truncate (Variables|Game|GetCurrency)))
  (Variables|/Script/Engine.PlayerController|SetbShowMouseCursor (Game|GetPlayerController 0) true) ; TEMP FOR MOUSE
)

(fn AddOrder
  (if (< (Variables|DayOrders|GetOrdersSent) (Variables|DayOrders|GetDayNumberOfOrders))
    (Default|AddRandomOrder (Variables|UIWidgets|GetHUDRef))
    (bind _returnvalue (Utilities|Time|SetTimerbyFunctionName 0 "AddOrder" (Variables|DayOrders|GetCurrentOrderDelay)))
    (Variables|DayOrders|SetOrderTimerHandle _returnvalue)
    (Math|Integer|IncrementInt (Variables|DayOrders|GetOrdersSent))
    (else
      (Utilities|Time|ClearandInvalidateTimerbyHandle (Variables|DayOrders|GetOrderTimerHandle)))))

(fn RestartGame
  (CallFunction|ResettoStartStas)
  (Game|SetGamePaused false)
  (CallFunction|NewDay)
  (CallFunction|DisplayEndScreen false)
  (CallFunction|AllPlayersDropActors)
  (CallFunction|RemoveAllPartsItemsandMats)
  (CallFunction|RestartPlayers)
  (Audio|PlaySound2D (Variables|Default|GetBackgroundSound) 0.3))

(fn DisplayEndScreen
  (params (Visible :type Boolean))
  (bind _returnvalue (Game|GetPlayerController 0))
  (Utilities|IsValid (Variables|UIWidgets|GetEnd%20Screen)
    (:Is%20Valid
      _)
    (:Is%20Not%20Valid
      (bind _returnvalue_2 (UserInterface|CreateWidget "/Game/UI/Screens/W_EndScreen.W_EndScreen_C"))
      (UserInterface|Viewport|AddtoViewport _returnvalue_2 0)
      (Variables|UIWidgets|SetEnd%20Screen _returnvalue_2)))
  (if Visible
    (Widget|SetVisibility (Variables|UIWidgets|GetEnd%20Screen) "Visible")
    (Input|SetInputModeUIOnly _returnvalue _returnvalue_2 "DoNotLock")
    (else
      (Widget|SetVisibility (Variables|UIWidgets|GetEnd%20Screen) "Hidden")
      (Input|SetInputModeGameOnly _returnvalue))))

(fn RemoveAllPartsItemsandMats
  (bind _outactors (Actor|GetAllActorsOfClass "/Script/UnderForge.ForgePart"))
  (for _array_element _outactors
    (Actor|DestroyActor _array_element))
  (bind _outactors_2 (Actor|GetAllActorsOfClass "/Script/UnderForge.ForgeMat"))
  (for _array_element_2 _outactors_2
    (Actor|DestroyActor _array_element_2))
  (bind _outactors_3 (Actor|GetAllActorsOfClass "/Script/UnderForge.ForgeItem"))
  (for _array_element_3 _outactors_3
    (Actor|DestroyActor _array_element_3)))

(fn AllPlayersDropActors
  (for _index (range 0 (- (Variables|Default|GetNumberOfPlayers) 1))
    (bind _asbp_forge_player (Utilities|Casting|CastToBP_ForgePlayer (Game|GetPlayerCharacter _index)))
    (Default|Drop _asbp_forge_player)))

(fn RestartPlayers
  (for _array_element (Variables|Default|GetCurrentPlayerControllers)
    (Utilities|IsValid _array_element
      (:Is%20Valid
        (Class|GameModeBase|RestartPlayer _array_element))))
  (Default|SetControllersView (Variables|Default|GetCameraControllerRef)))

(fn OrderExpired)

(fn TogglePauseGame
  (CallFunction|SetGamePaused (not (Game|IsGamePaused))))

(fn SetGamePaused
  (params (IsPaused :type Boolean))
  (bind _returnvalue (Game|GetPlayerController 0))
  (bind _pausescreen (Variables|UIWidgets|GetPauseScreen))
  (Game|SetGamePaused IsPaused)
  (if IsPaused
    (Widget|SetVisibility _pausescreen "Visible")
    (Input|SetInputModeGameandUI _returnvalue (Variables|/Game/UI/Screens/W_PauseScreen.W_PauseScreen_C|GetResume _pausescreen) "DoNotLock" false)
    (Variables|/Script/Engine.PlayerController|SetbShowMouseCursor _returnvalue true)
    (else
      (Widget|SetVisibility _pausescreen "Hidden")
      (Input|SetInputModeGameOnly _returnvalue)
      (Variables|/Script/Engine.PlayerController|SetbShowMouseCursor _returnvalue false))))

(fn AddandRemovePlayers
  (bind _currentcontrollerid (LocalVariables|GetCurrentControllerID))
  (bind _currentplayercontrollers (Variables|Default|GetCurrentPlayerControllers))
  ;[1 1 1] Spawn extra players
  (for (_array_element _array_index) (Variables|/Game/Blueprints/Mechanics/ForgeGameInstance.ForgeGameInstance_C|GetPlayerState (Variables|Default|GetGameInstanceRef))
    (if _array_element
      (Utilities|IsValid (Game|GetPlayerController _array_index)
        (:Is%20Not%20Valid
          (Class|GameplayStatics|CreatePlayer _array_index)))))
  ;[1 1 1] Get Number of Players
  (for _array_element_2 (Variables|/Game/Blueprints/Mechanics/ForgeGameInstance.ForgeGameInstance_C|GetPlayerState (Variables|Default|GetGameInstanceRef))
    (if _array_element_2
      (Math|Integer|IncrementInt (Variables|Default|GetNumberOfPlayers))))
  ;[1 1 1] Remove Extra Players (Above Count)
  (for _index (range (Variables|Default|GetNumberOfPlayers) 3)
    (Utilities|IsValid (Game|GetPlayerController _index)
      (:Is%20Valid
        ;;[1 1 1] Has to be Twice? thanks unreal
        (Class|GameplayStatics|RemovePlayer (Game|GetPlayerController _index) true)
        (Class|GameplayStatics|RemovePlayer (Game|GetPlayerController _index) true))))
  ;[1 1 1] Set Controller IDs
  (for _index_2 (range 0 3)
    (if (Utilities|Array|Get(acopy) (Variables|/Game/Blueprints/Mechanics/ForgeGameInstance.ForgeGameInstance_C|GetPlayerState (Variables|Default|GetGameInstanceRef)) _index_2)
      (Class|GameplayStatics|SetPlayerControllerID (Game|GetPlayerController _currentcontrollerid) _index_2)
      (Math|Integer|IncrementInt _currentcontrollerid)))
  ;[1 1 1] Add To Controllers Array
  (Utilities|Array|Clear _currentplayercontrollers)
  (for _index_3 (range 0 3)
    (bind _asforge_controller (Utilities|Casting|CastToForgeController (Game|GetPlayerController _index_3)))
    (Utilities|Array|Add _currentplayercontrollers _asforge_controller))
  (Utilities|PrintCurrentPlayerswithIDs))

(fn ResettoStartStas
  (bind _initialstatvalues (Variables|Default|GetInitialStatValues))
  (bind (_daytime _daytimeincreaserate _numberoforders _orderincreaserate) (Utilities|Struct|BreakStartStats _initialstatvalues))
  (Variables|DayCycle|SetCurrentDay 0)
  (Variables|DayCycle|SetDayTime _daytime)
  (Variables|DayCycle|SetDayTimeIncreaseRate _daytimeincreaserate)
  (Variables|DayOrders|SetDayNumberOfOrders _numberoforders)
  (Variables|DayOrders|SetOrderIncreaseRate _orderincreaserate))