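; Player controller for the menu that lets players join or leave by controller ID and start the game.
; Enter or gamepad bottom face button adds the player, L or right face button removes them, and the Menu action starts the game, all through GM_MenuGameMode.
; SetHostScreen and SetJoinScreen lazily create, cache and show or hide the Host and Join widgets, focusing a button when shown.
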(event EventBeginPlay
  (bind _asgm_menu_game_mode (Utilities|Casting|CastToGM_MenuGameMode (Game|GetGameMode)))
  (Variables|Default|SetGameModeRef _asgm_menu_game_mode))

(event EventTick
  (params (DeltaSeconds :type Float%20%28single-precision%29)))

(event Input|ActionEvents|InputActionMenu
  (params (Key :type Key%20Structure :default "None"))
  (:Pressed
    (Default|StartGame (Variables|Default|GetGameModeRef))))

(event Input|KeyboardEvents|L
  (params (Key :type Key%20Structure :default "None"))
  (:Pressed
    (Default|RemovePlayer (Variables|Default|GetGameModeRef) (Class|GameplayStatics|GetPlayerControllerID self))))

(event Input|KeyboardEvents|Enter
  (params (Key :type Key%20Structure :default "None"))
  (bind _self self)
  (bind _returnvalue (Class|GameplayStatics|GetPlayerControllerID _self))
  (:Pressed
    (Development|PrintString (Utilities|String|Append "Player " (Utilities|String|ToString(Integer) _returnvalue) " pressing A"))
    (Default|SetPlayer (Variables|Default|GetGameModeRef) _returnvalue)))

(event Input|GamepadEvents|GamepadFaceButtonBottom
  (params (Key :type Key%20Structure :default "None"))
  (bind _self self)
  (bind _returnvalue (Class|GameplayStatics|GetPlayerControllerID _self))
  (:Pressed
    (Development|PrintString (Utilities|String|Append "Player " (Utilities|String|ToString(Integer) _returnvalue) " pressing A"))
    (Default|SetPlayer (Variables|Default|GetGameModeRef) _returnvalue)))

(event Input|GamepadEvents|GamepadFaceButtonRight
  (params (Key :type Key%20Structure :default "None"))
  (:Pressed
    (Default|RemovePlayer (Variables|Default|GetGameModeRef) (Class|GameplayStatics|GetPlayerControllerID self))))

(fn ConstructionScript)

(fn SetHostScreen
  (params (Visible :type Boolean))
  (if Visible
    (Utilities|IsValid (Variables|Default|GetHostWidget)
      (:Is%20Valid
        (Widget|SetVisibility (Variables|Default|GetHostWidget) "Visible"))
      (:Is%20Not%20Valid
        (bind _returnvalue (UserInterface|CreateWidget "/Game/UI/MainMenu/W_Host.W_Host_C" self))
        (bind _output_get (Variables|Default|SetHostWidget _returnvalue))
        (UserInterface|Viewport|AddtoViewport _output_get 0)))
    (Class|Widget|SetUserFocus (Variables|/Game/UI/MainMenu/W_Host.W_Host_C|GetHostBtn _output_get) self)
    (else
      (Utilities|IsValid (Variables|Default|GetHostWidget)
        (:Is%20Valid
          (Widget|SetVisibility (Variables|Default|GetHostWidget) "Hidden"))))))

(fn SetJoinScreen
  (params (Visible :type Boolean))
  (if Visible
    (Utilities|IsValid (Variables|Default|GetJoinWidget)
      (:Is%20Valid
        (Widget|SetVisibility (Variables|Default|GetJoinWidget) "Visible"))
      (:Is%20Not%20Valid
        (bind _returnvalue (UserInterface|CreateWidget "/Game/UI/MainMenu/W_Join.W_Join_C" self))
        (bind _output_get (Variables|Default|SetJoinWidget _returnvalue))
        (UserInterface|Viewport|AddtoViewport _output_get 0)))
    (Class|Widget|SetUserFocus (Variables|/Game/UI/MainMenu/W_Join.W_Join_C|GetCreateBtn _output_get) self)
    (else
      (Utilities|IsValid (Variables|Default|GetJoinWidget)
        (:Is%20Valid
          (Widget|SetVisibility (Variables|Default|GetJoinWidget) "Hidden"))))))