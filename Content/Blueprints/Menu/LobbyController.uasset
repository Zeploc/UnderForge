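; Lobby player controller that runs the ready screen, music and camera backdrop before a multiplayer game starts.
; On local BeginPlay it creates the Ready widget, switches view to a level CameraActor and plays a Matinee.
; Interact sends ready toggles to GM_Lobby via a server event, while MULTI events update or remove the widget.
; Menu asks the game mode to start; Throw destroys the session and opens MainMenu.
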(event Custom|MULTI_SetPlayerReady
  (params (Player :type Player%20State%20Object%20Reference) (Ready :type Boolean))
  (bind _readyscreenwidget (CallFunction|GetPlayerScreen))
  (if (Pawn|IsLocalPlayerController)
    (Utilities|IsValid _readyscreenwidget
      (:Is%20Valid
        (Default|SetPlayerReady _readyscreenwidget Player Ready)))))

(event Custom|SERVER_ChangedReady
  (params (Ready :type Boolean%20%28by%20ref%29))
  (Default|SetPlayer (Variables|Default|GetLobbyGameModeRef) (Variables|Default|GetPlayerState) Ready))

(event Custom|MULTI_RemovePlayer
  (params (Player :type Player%20State%20Object%20Reference%20%28by%20ref%29))
  (bind _readyscreenwidget (CallFunction|GetPlayerScreen))
  (if (Pawn|IsLocalPlayerController)
    (Utilities|IsValid _readyscreenwidget
      (:Is%20Valid
        (Default|RemovePlayer _readyscreenwidget Player)))))

(event Custom|MULTI_JoiningGame
  (Widget|RemovefromParent (Variables|Default|GetReadyScreenWidget)))

(event EventBeginPlay
  (bind _asgm_lobby (Utilities|Casting|CastToGM_Lobby (Game|GetGameMode))
    (:then
      (Variables|Default|SetLobbyGameModeRef _asgm_lobby))
    (:CastFailed
      _))
  (if (Pawn|IsLocalPlayerController)
    (Audio|PlaySound2D (Variables|Default|GetLobbyMusic) 1.0 1.0 0.0 0 0)
    (CallFunction|DisplayPlayerScreen)
    (bind _returnvalue (Actor|GetActorOfClass "/Script/Engine.CameraActor"))
    (Game|Player|SetViewTargetwithBlend _returnvalue 0.0 "VTBlend_Linear" 0.0 false)
    (bind _returnvalue_2 (Actor|GetActorOfClass "/Script/Engine.MatineeActor"))
    (Audio|Components|Audio|Play _returnvalue_2)))

(event EventTick
  (params (DeltaSeconds :type Float%20%28single-precision%29)))

(event Input|ActionEvents|InputActionThrow
  (params (Key :type Key%20Structure :default "None"))
  (:Pressed
    (|DestroySession self
      (:OnSuccess
        _)
      (:OnFailure
        _))
    (Game|OpenLevel(byName) "MainMenu")))

(event Input|ActionEvents|InputActionMenu
  (params (Key :type Key%20Structure :default "None"))
  (bind _lobbygamemoderef (Variables|Default|GetLobbyGameModeRef))
  (:Pressed
    (Utilities|IsValid _lobbygamemoderef
      (:Is%20Valid
        (Default|StartGame _lobbygamemoderef)))))

(event Input|ActionEvents|InputActionInteract
  (params (Key :type Key%20Structure :default "None"))
  (:Pressed
    (Development|PrintString (Utilities|String|Append "Player " (Utilities|String|ToString(Integer) (Class|GameplayStatics|GetPlayerControllerID self)) " pressing A"))
    (bind _output_get (Variables|Default|SetCurrentReady (not (Variables|Default|GetCurrentReady))))
    (CallFunction|SERVERChangedReady _output_get)))

(fn ConstructionScript)

(fn DisplayPlayerScreen
  (Utilities|IsValid (Variables|Default|GetReadyScreenWidget)
    (:Is%20Valid
      (Widget|SetVisibility (Variables|Default|GetReadyScreenWidget) "Visible"))
    (:Is%20Not%20Valid
      (bind _returnvalue (UserInterface|CreateWidget "/Game/UI/MainMenu/Ready.Ready_C" (Game|GetPlayerController 0)))
      (bind _output_get (Variables|Default|SetReadyScreenWidget _returnvalue))
      (UserInterface|Viewport|AddtoViewport _output_get 0)
      (Input|SetInputModeGameandUI self 0 "DoNotLock" true))))

(fn GetPlayerScreen
  (Utilities|IsValid (Variables|Default|GetReadyScreenWidget)
    (:Is%20Valid
      _)
    (:Is%20Not%20Valid
      (CallFunction|DisplayPlayerScreen)))
  (return (Variables|Default|GetReadyScreenWidget)))