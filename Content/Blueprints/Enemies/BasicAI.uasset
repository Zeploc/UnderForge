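; Basic enemy AI character that moves toward the Smeltery in the level.
; BeginPlay caches the first BP_Smeltery found, and Tick reissues a simple move-to-actor toward it every frame.
; A RayCastCheck helper box-traces forward from the lowered capsule position by a given distance and channel, branching to Hit with the actor or Missed.
; The helper is not called in this graph.
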(event EventTick
  (params (DeltaSeconds :type Float%20%28single-precision%29))
  (AI|Navigation|SimpleMovetoActor (Pawn|GetController self) (Variables|Default|GetSmelteryRef)))

(event EventBeginPlay
  (bind _outactors (Actor|GetAllActorsOfClass "/Game/Blueprints/LevelBlueprints/BP_Smeltery.BP_Smeltery_C"))
  (Variables|Default|SetSmelteryRef (Utilities|Array|Get(acopy) _outactors)))

(fn ConstructionScript)