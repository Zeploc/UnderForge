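; Base enemy character that walks to the smeltery and damages its forge, with a health bar widget.
; Tick drives movement while SmelteryRef is valid, plays timer-gated attack montages whose "Attack" notify deals damage, and destroys the actor at zero health.
; TakeDamage applies mass-scaled knockback and a brief stun that pauses movement orders, plus sound, particles and floating damage numbers.
; RayCastCheck is a forward box-trace helper.
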(event EventTick
  (params (DeltaSeconds :type Float%20%28single-precision%29))
  (bind _smelteryref (Variables|Default|GetSmelteryRef))
  (Utilities|IsValid (Variables|Default|GetSmelteryRef)
    (:Is%20Valid
      (if (<= (Variables|Default|GetHealth) 0)
        (Actor|DestroyActor)
        (elif (Variables|Default|GetStunned)
          (Variables|Default|SetHitForge false)
          (Utilities|FlowControl|Delay 0.2)
          (Variables|Default|SetStunned false)
          (else
            (AI|Navigation|SimpleMovetoActor (Pawn|GetController self) _smelteryref)
            (if (< (Math|Vector|VectorLength (- (Transformation|GetActorLocation) (Transformation|GetActorLocation _smelteryref))) (Variables|Default|GetForgeAttackRange))
              (if (not (Variables|Default|GetHitForge))
                (Variables|Default|SetHitForge true)
                (Utilities|Time|SetTimerbyFunctionName 0 "ResetCanDamageForge" (Variables|Default|GetDamageTime))
                (bind _notifyname (Animation|Montage|PlayMontage (Variables|Character|GetMesh) (Variables|Default|GetAttackMontage))
                  (:OnNotifyBegin
                    (if (Utilities|Name|Equal(Name) _notifyname "Attack")
                      (if (Variables|Default|GetHitForge)
                        (Class|Smeltery|DamageForge (Variables|Default|GetSmelteryRef) (Variables|Default|GetDamageToForge))))))))))))))

(event EventBeginPlay
  (Variables|Default|SetMaxHealth (Variables|Default|GetHealth))
  (Audio|PlaySound2D (Variables|Sounds|GetSpawnSound) 0.4 1.0 0.0 0 0)
  (bind _asw_enemy_health_bar (Utilities|Casting|CastToW_EnemyHealthBar (UserInterface|GetUserWidgetObject (Variables|Default|GetHealthWidget))))
  (Variables|/Game/UI/Enemies/W_EnemyHealthBar.W_EnemyHealthBar_C|SetEnemy _asw_enemy_health_bar self))

(fn ConstructionScript)

(fn TakeDamage
  (params (Damage :type Integer) (Location :type Vector) (Crit :type Boolean) (KnockbackMultiplier :type Float%20%28single-precision%29))
  (bind _returnvalue (Transformation|GetActorLocation))
  (Variables|Default|SetHealth (- (Variables|Default|GetHealth) Damage))
  (bind _output_get (Variables|Default|SetForce (- (Transformation|GetActorLocation) Location)))
  (bind _output_get_2 (Variables|Default|SetForce (Math|Vector|Normalize _output_get)))
  (bind _output_get_3 (Variables|Default|SetForce (* _output_get_2 (/ (* (* Damage KnockbackMultiplier) 25.0) (Math|Conversions|ToFloat(Integer) (Variables|Default|GetMass))))))
  (Variables|Default|SetStunned true)
  (Character|LaunchCharacter _output_get_3 true true)
  (Components|Movement|StopMovementImmediately (Variables|Character|GetCharacterMovement))
  (Audio|PlaySoundatLocation (select Crit (Variables|Default|GetCritHitSound) (Variables|Sounds|GetHitSound)) (Transformation|GetActorLocation) "0, 0, 0" 0.6 1.0 0.0 0 0 0)
  (bind _returnvalue_2 (Game|SpawnActorfromClass "/Game/Blueprints/Enemies/DamageDisplay.DamageDisplay_C" (Transformation|GetActorTransform) "AlwaysSpawn" self 0))
  (Transformation|AttachActorToActor _returnvalue_2 self "None" "KeepWorld" "KeepWorld" "KeepRelative" true)
  (bind _asw_damage_display (Utilities|Casting|CastToW_DamageDisplay (UserInterface|GetUserWidgetObject (Variables|/Game/Blueprints/Enemies/DamageDisplay.DamageDisplay_C|GetDamageWidget _returnvalue_2))))
  (Default|SetDamage _asw_damage_display (Math|Conversions|ToFloat(Integer) Damage) Crit)
  (Effects|SpawnEmitteratLocation "/Game/Effects/HitParticle/Hit_P.Hit_P" (+ _returnvalue (* (Math|Vector|Normalize (- Location _returnvalue)) 5e+01))))

(fn ResetCanDamageForge
  (Variables|Default|SetHitForge false))