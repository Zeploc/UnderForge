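; Server-side enemy wave manager that spawns the current level's waves, looked up by level name in the Forge game instance.
; Chained NewWave timers advance waves, while a looping timer spawns each enemy at the manager's location, facing the Smeltery and holding a reference to it.
; Wave countdowns are multicast through ForgeGameState, and GM_ForgeLevel checks day completion once the wave index runs past the list.
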(event EventBeginPlay
  (Networking|SwitchHasAuthority
    (:Authority
      (bind _returnvalue (Game|GetCurrentLevelName true))
      (if (.ReturnValue (Utilities|Map|Find (Variables|/Game/Blueprints/Gameplay/ForgeGameInstance.ForgeGameInstance_C|GetLevels (CallFunction|GetForgeGameInstance)) _returnvalue))
        (Variables|Default|SetCurrentWaves (.Waves (Utilities|Struct|BreakLevelSet (.Value (Utilities|Map|Find (Variables|/Game/Blueprints/Gameplay/ForgeGameInstance.ForgeGameInstance_C|GetLevels (CallFunction|GetForgeGameInstance)) _returnvalue)))))
        (bind _returnvalue_2 (Utilities|Time|SetTimerbyFunctionName 0 "NewWave" (.InitialDelayTillWaves (Utilities|Struct|BreakLevelSet (.Value (Utilities|Map|Find (Variables|/Game/Blueprints/Gameplay/ForgeGameInstance.ForgeGameInstance_C|GetLevels (CallFunction|GetForgeGameInstance)) _returnvalue))))))
        (bind _output_get (Variables|Default|SetWaveHandle _returnvalue_2))
        (CallFunction|UpdateGamestateTimer (Utilities|Time|GetTimerRemainingTimebyHandle _output_get))
        (Utilities|IsValid (Variables|Default|GetSmeltery)
          (:Is%20Not%20Valid
            (bind _returnvalue_3 (Actor|GetActorOfClass "/Game/Blueprints/LevelBlueprints/BP_Smeltery.BP_Smeltery_C"))
            (Utilities|IsValid _returnvalue_3
              (:Is%20Valid
                (Variables|Default|SetSmeltery _returnvalue_3)))))
        (else
          (Development|PrintString "NO WAVES FOUND" true true "(R=1.000000,G=0.027472,B=0.000000,A=1.000000)" 5.0))))))

(event Collision|EventActorBeginOverlap
  (params (OtherActor :type Actor%20Object%20Reference)))

(event EventTick
  (params (DeltaSeconds :type Float%20%28single-precision%29)))

(fn ConstructionScript)

(fn SpawnEnemies
  (bind _waveindex (Variables|Default|GetWaveIndex))
  (bind _waveenemyindex (Variables|Default|GetWaveEnemyIndex))
  (bind _currentwaves (Variables|Default|GetCurrentWaves))
  (bind _output (Utilities|Array|Get(acopy) _currentwaves _waveindex))
  (if (>= _waveenemyindex (Utilities|Array|Length (.enemies _output)))
    (Utilities|Time|ClearandInvalidateTimerbyHandle (Variables|Default|GetEnemySpawningHandle))
    (else
      (LocalVariables|SetNewClass (Utilities|Array|Get(acopy) (.enemies _output) _waveenemyindex))
      (Math|Integer|IncrementInt (Variables|Default|GetWaveEnemyIndex)
        (:%20%20
          (LocalVariables|SetSpawnLoc (Transformation|GetActorLocation))
          (bind _returnvalue (AI|SpawnAIFromClass (LocalVariables|GetNewClass) 0 (LocalVariables|GetSpawnLoc) (Math|Rotator|FindLookatRotation (LocalVariables|GetSpawnLoc) (Transformation|GetActorLocation (Variables|Default|GetSmeltery))) false 0))
          (bind _asenemy_base (Utilities|Casting|CastToEnemyBase _returnvalue))
          (Variables|/Game/Blueprints/Enemies/EnemyBase.EnemyBase_C|SetSmelteryRef _asenemy_base (Variables|Default|GetSmeltery)))))))

(fn NewWave
  (bind _currentwaves (Variables|Default|GetCurrentWaves))
  (bind _waveindex (Variables|Default|GetWaveIndex))
  (bind _output (Utilities|Array|Get(acopy) _currentwaves _waveindex))
  (bind _delaytillnextwave (Utilities|Struct|BreakWave _output))
  (Math|Integer|IncrementInt (Variables|Default|GetWaveIndex)
    (:%20%20
      (Variables|Default|SetWaveEnemyIndex 0)
      (CallFunction|SpawnEnemies)
      (bind _returnvalue (Utilities|Time|SetTimerbyFunctionName 0 "SpawnEnemies" 1.0 true))
      (Variables|Default|SetEnemySpawningHandle _returnvalue)
      (if (< (Variables|Default|GetWaveIndex) (Utilities|Array|Length (Variables|Default|GetCurrentWaves)))
        (bind _returnvalue_2 (Utilities|Time|SetTimerbyFunctionName 0 "NewWave" _delaytillnextwave))
        (Variables|Default|SetWaveHandle _returnvalue_2)
        (CallFunction|UpdateGamestateTimer _delaytillnextwave)
        (else
          (Utilities|Time|ClearandInvalidateTimerbyHandle (Variables|Default|GetWaveHandle))
          (bind _asgm_forge_level (Utilities|Casting|CastToGM_ForgeLevel (Game|GetGameMode)))
          (Default|CheckDayComplete _asgm_forge_level))))))

(fn GetForgeGameInstance
  (Utilities|IsValid (Variables|Default|GetForgeGameInstance)
    (:Is%20Valid
      _)
    (:Is%20Not%20Valid
      (bind _asforge_game_instance (Utilities|Casting|CastToForgeGameInstance (Game|GetGameInstance)))
      (Variables|Default|SetForgeGameInstance _asforge_game_instance)))
  (return (Variables|Default|GetForgeGameInstance)))

(fn GetCurrentWaveTime
  (bind _wavehandle (Variables|Default|GetWaveHandle))
  (if (Utilities|Time|IsValidTimerHandle _wavehandle)
    (return (+ (Class|KismetSystemLibrary|GetTimerElapsedTimeHandle _wavehandle) (Utilities|Time|GetTimerRemainingTimebyHandle _wavehandle)))
    (else
      (return 0.0))))

(fn UpdateGamestateTimer
  (params (NewTime :type Float%20%28single-precision%29))
  (bind _forgegamestate (CallFunction|GetForgeGameState))
  (Utilities|IsValid _forgegamestate
    (:Is%20Valid
      (Default|MULTIStartWaveTimer _forgegamestate NewTime))))

(fn GetForgeGameState
  (Utilities|IsValid (Variables|Default|GetForgeGameState)
    (:Is%20Valid
      _)
    (:Is%20Not%20Valid
      (bind _asforge_game_state (Utilities|Casting|CastToForgeGameState (Game|GetGameState)))
      (Variables|Default|SetForgeGameState _asforge_game_state)))
  (return (Variables|Default|GetForgeGameState)))