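; Customer character that walks to goal locations and carries a weapon it receives away to the customer manager's spawn point.
; SetGoalLocation issues an AI simple move and caches the goal.
; TakeWeapon attaches the weapon to a finger socket using its attach offset, disables its physics and collision, then sends the customer to the spawn point.
; Once holding a weapon, Tick destroys both weapon and customer near the goal.
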(event EventBeginPlay)

(event Collision|EventActorBeginOverlap
  (params (OtherActor :type Actor%20Object%20Reference)))

(event EventTick
  (params (DeltaSeconds :type Float%20%28single-precision%29))
  (Utilities|IsValid (Variables|Default|GetCurrentWeapon)
    (:Is%20Valid
      (if (<= (Math|Vector|VectorLength (- (Variables|Default|GetGoaLoc) (Transformation|GetActorLocation))) 1.5e+02)
        (Actor|DestroyActor (Variables|Default|GetCurrentWeapon))
        (Actor|DestroyActor)))))

(fn ConstructionScript)

(fn SetGoalLocation
  (params (GoalLocation :type Vector))
  (AI|Navigation|SimpleMovetoLocation (AI|GetAIController self) GoalLocation)
  (Variables|Default|SetGoaLoc GoalLocation))

(fn TakeWeapon
  (params (Weapon :type Sword%20Item%20Object%20Reference) (CustomerManager :type Customer%20Manager%20Object%20Reference))
  (bind _itemmesh (Variables|/Script/UnderForge.PickUpItem|GetItemMesh Weapon))
  (Transformation|SetActorRelativeTransform Weapon (Variables|/Script/UnderForge.PickUpItem|GetAttachOffset Weapon) false false)
  (Transformation|AttachComponentToComponent Weapon (Variables|Character|GetMesh) "MiddleFinger2_R" "KeepRelative" "KeepRelative" "KeepRelative" false)
  (CallFunction|SetGoalLocation (Transformation|GetWorldLocation (Variables|/Game/Blueprints/Customers/CustomerManager.CustomerManager_C|GetSpawnLocation CustomerManager)))
  (Physics|SetSimulatePhysics _itemmesh false)
  (Collision|SetCollisionProfileName _itemmesh "NoCollision" true :!class /Script/Engine.PrimitiveComponent)
  (Variables|Default|SetCurrentWeapon Weapon))