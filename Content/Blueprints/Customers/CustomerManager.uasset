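; CustomerManager spawns AI customers for a sword forge game and keeps them in an ordered array that acts as a queue.
; NewCustomer spawns a Customer_BP at the SpawnLocation component and sets the manager's own location as its goal.
; GiveToCustomer locks a handed-in sword, makes it drop from any holder, passes it to the front customer and dequeues them.
; RemoveAllCustomers destroys and clears the queue.
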(event EventBeginPlay)

(event Collision|EventActorBeginOverlap
  (params (OtherActor :type Actor%20Object%20Reference)))

(event EventTick
  (params (DeltaSeconds :type Float%20%28single-precision%29)))

(fn ConstructionScript)

(fn NewCustomer
  (bind _spawnlocation (Variables|Default|GetSpawnLocation))
  (bind _returnvalue (AI|SpawnAIFromClass "/Game/Blueprints/Customers/Customer_BP.Customer_BP_C" 0 (Transformation|GetWorldLocation _spawnlocation) (Transformation|GetWorldRotation _spawnlocation) false 0))
  (bind _ascustomer_bp (Utilities|Casting|CastToCustomer_BP _returnvalue))
  (Utilities|Array|Add (Variables|Default|GetCustomers) _ascustomer_bp)
  (Default|SetGoalLocation _ascustomer_bp (Transformation|GetActorLocation)))

(fn GivetoCustomer
  (params (Sword :type Sword%20Item%20Object%20Reference))
  (bind _heldplayer (Variables|/Script/UnderForge.PickUpItem|GetHeldPlayer Sword))
  (Utilities|FlowControl|Sequence
    (:then_0
      (bind _asbp_sword (Utilities|Casting|CastToBP_Sword Sword))
      (Variables|/Game/Blueprints/ItemsBlueprints/BP_Sword.BP_Sword_C|SetHandedIn _asbp_sword true)
      (Variables|/Script/UnderForge.PickUpItem|SetCanBePickedUp _asbp_sword false))
    (:then_1
      (Utilities|IsValid _heldplayer
        (:Is%20Valid
          (bind _asbp_forge_player (Utilities|Casting|CastToBP_ForgePlayer _heldplayer)
            (:then
              (Default|MULTIDrop _asbp_forge_player))
            (:CastFailed
              (Class|PickUpItem|Drop Sword :!label _label))))
        (:Is%20Not%20Valid
          (goto _label)))
      (Default|TakeWeapon (Utilities|Array|Get(acopy) (Variables|Default|GetCustomers)) Sword self)
      (Utilities|Array|RemoveIndex (Variables|Default|GetCustomers)))))

(fn RemoveAllCustomers
  (bind _customers (Variables|Default|GetCustomers))
  (for _array_element _customers
    (Actor|DestroyActor _array_element))
  (Utilities|Array|Clear _customers))