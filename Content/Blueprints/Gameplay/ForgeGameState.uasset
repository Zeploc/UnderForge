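; Game state for a forge level that manages weapon orders and relays order, currency, wave timer and end-of-day events to players.
; The server adds random orders from the level's weapon set on a looping timer, multicasting them to each local ForgeControllerBP and spawning customers via CustomerManager.
; ProcessItem matches a sword to an open order, completes it through GM_ForgeLevel with its durability ratio, and gives it to a customer.
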(event Custom|MULTI_NewOrder
  (params (Weapon :type EWeapon%20Enum :default "W_NONE") (ID :type Integer%20%28by%20ref%29))
  (bind _returnvalue (Game|GetPlayerController 0))
  (if (Pawn|IsLocalPlayerController _returnvalue)
    (bind _asforge_controller_bp (Utilities|Casting|CastToForgeControllerBP _returnvalue))
    (Default|NewOrder _asforge_controller_bp Weapon ID)
    (Development|PrintString (Utilities|String|Append "New Order " (Utilities|String|ToString(Integer) ID)) false true "(R=1.000000,G=0.731737,B=0.237019,A=1.000000)" 1e+01)))

(event Custom|MULTI_CompleteOrder
  (params (OrderID :type Integer))
  (bind _returnvalue (Game|GetPlayerController 0))
  (if (Pawn|IsLocalPlayerController _returnvalue)
    (bind _asforge_controller_bp (Utilities|Casting|CastToForgeControllerBP _returnvalue))
    (Default|CompleteOrder _asforge_controller_bp OrderID)))

(event Custom|S_SendOutOrders
  (Networking|SwitchHasAuthority
    (:Authority
      (bind _keys (Utilities|Map|Keys (Variables|Default|GetOrders)))
      (for _array_element _keys
        (CallFunction|MULTINewOrder (.Value (Utilities|Map|Find (Variables|Default|GetOrders) _array_element)) _array_element)))))

(event Custom|MULTI_TEST
  (Development|PrintString "Hello"))

(event Custom|MULTI_StartWaveTimer
  (params (Time :type Float%20%28single-precision%29))
  (bind _returnvalue (Utilities|Time|SetTimerbyEvent (delegate Custom|ClearTimer) Time))
  (Variables|Default|SetWaveTimer _returnvalue))

(event Custom|ClearTimer
  (Utilities|Time|ClearandInvalidateTimerbyHandle (Variables|Default|GetWaveTimer)))

(event Custom|MULTI_GainedCurrency
  (params (Gained :type Integer) (NewVal :type Integer))
  (CallFunction|GainedCurrency Gained NewVal))

(event Custom|GetUpdateWaveTimer
  (bind _asforge_controller_bp (Utilities|Casting|CastToForgeControllerBP (Game|GetPlayerController 0)))
  (Default|SERVERUpdateWaveTimer _asforge_controller_bp))

(event Custom|MULTI_EndDay
  (params (Currency :type Integer) (CurrencyNeeded :type Integer) (ForgeHealth :type Float%20%28single-precision%29))
  (bind _asforge_controller_bp (Utilities|Casting|CastToForgeControllerBP (Game|GetPlayerController 0)))
  (Default|EndRoundScreen _asforge_controller_bp Currency CurrencyNeeded ForgeHealth)
  (Utilities|Time|PauseTimerbyHandle (Variables|Default|GetWaveTimer)))

(event EventBeginPlay
  (bind _returnvalue (Actor|GetActorOfClass "/Game/Blueprints/Customers/CustomerManager.CustomerManager_C"))
  (Variables|Default|SetCustomerManager _returnvalue)
  (Networking|SwitchHasAuthority
    (:Authority
      _)
    (:Remote
      (CallFunction|GetUpdateWaveTimer)))
  (Utilities|FlowControl|Delay 3.0)
  (Networking|SwitchHasAuthority
    (:Authority
      (CallFunction|MULTITEST))))

(event EventTick
  (params (DeltaSeconds :type Float%20%28single-precision%29))
  (bind _forgegm (CallFunction|GetGamemode))
  (Networking|SwitchHasAuthority
    (:Authority
      (Utilities|IsValid _forgegm
        (:Is%20Valid
          (Variables|Default|SetDayTimeRemaining (Utilities|Time|GetTimerRemainingTimebyHandle (Variables|/Game/Blueprints/Gameplay/GM_ForgeLevel.GM_ForgeLevel_C|GetDayTimerHandle _forgegm))))))))

(fn ConstructionScript)

(fn RemoveAllOrders
  (bind _customermanager (CallFunction|GetCustomerManager))
  (Utilities|Map|Clear (Variables|Default|GetOrders))
  (Utilities|IsValid _customermanager
    (:Is%20Valid
      (Default|RemoveAllCustomers _customermanager))))

(fn AddBeginningOrders
  (bind _forgegm (CallFunction|GetGamemode))
  (CallFunction|RemoveAllOrders)
  (Utilities|IsValid _forgegm
    (:Is%20Valid
      (for _index (range 0 (Variables|/Game/Blueprints/Gameplay/GM_ForgeLevel.GM_ForgeLevel_C|GetBeginningNumberOfOrders _forgegm))
        (CallFunction|SAddRandomOrder))
      (bind _returnvalue (Utilities|Time|SetTimerbyFunctionName 0 "S_AddRandomOrder" (Variables|/Game/Blueprints/Gameplay/GM_ForgeLevel.GM_ForgeLevel_C|GetCurrentOrderDelay _forgegm) true))
      (Variables|Default|SetOrdersHandle _returnvalue))))

(fn SAddRandomOrder
  (bind _customermanager (CallFunction|GetCustomerManager))
  (bind _weapons (CallFunction|GetAvailableWeapons))
  (bind _lastorderid (Variables|Default|GetLastOrderID))
  (Networking|SwitchHasAuthority
    (:Authority
      (Math|Integer|IncrementInt (Variables|Default|GetLastOrderID)
        (:%20%20
          (bind _output_get (LocalVariables|SetNewOrder (Utilities|Array|Get(acopy) _weapons (Math|Random|RandomInteger (Utilities|Array|Length _weapons)))))
          (Utilities|Map|Add (Variables|Default|GetOrders) _lastorderid _output_get)
          (CallFunction|MULTINewOrder (LocalVariables|GetNewOrder) _lastorderid)
          (Utilities|IsValid _customermanager
            (:Is%20Valid
              (Default|NewCustomer _customermanager))))))))

(fn GetGamemode
  (Utilities|IsValid (Variables|Default|GetForgeGM)
    (:Is%20Valid
      _)
    (:Is%20Not%20Valid
      (bind _asgm_forge_level (Utilities|Casting|CastToGM_ForgeLevel (Game|GetGameMode)))
      (Variables|Default|SetForgeGM _asgm_forge_level)))
  (return (Variables|Default|GetForgeGM)))

(fn CompleteOrder
  (params (OrderID :type Integer))
  (Utilities|Map|Remove (Variables|Default|GetOrders) OrderID)
  (CallFunction|MULTICompleteOrder OrderID))

(fn ProcessItem
  (params (Sword :type Sword%20Item%20Object%20Reference))
  (bind _forgegm (CallFunction|GetGamemode))
  (Utilities|FlowControl|Sequence
    (:then_0
      (bind _asbp_sword (Utilities|Casting|CastToBP_Sword Sword))
      (if (Variables|/Game/Blueprints/ItemsBlueprints/BP_Sword.BP_Sword_C|GetHandedIn _asbp_sword)
        (return)))
    (:then_1
      (Networking|SwitchHasAuthority
        (:Authority
          (bind _keys (Utilities|Map|Keys (Variables|Default|GetOrders)))
          (for _array_element _keys
            (if (Utilities|Enum|Equal(Enum) (Variables|/Script/UnderForge.SwordItem|GetWeaponType Sword) (.Value (Utilities|Map|Find (Variables|Default|GetOrders) _array_element)))
              (Utilities|IsValid _forgegm
                (:Is%20Valid
                  (bind _asbp_sword_2 (Utilities|Casting|CastToBP_Sword Sword)
                    (:then
                      (LocalVariables|SetDurability (/ (Math|Conversions|ToFloat(Integer) (Variables|/Game/Blueprints/ItemsBlueprints/BP_Sword.BP_Sword_C|GetDurability _asbp_sword_2)) (Math|Conversions|ToFloat(Integer) (Variables|/Game/Blueprints/ItemsBlueprints/BP_Sword.BP_Sword_C|GetMaxDurability _asbp_sword_2)))))
                    (:CastFailed
                      _))
                  (Default|CompleteOrder _forgegm _array_element (LocalVariables|GetDurability)))
                (:Is%20Not%20Valid
                  _))
              (bind _asbp_forge_player (Utilities|Casting|CastToBP_ForgePlayer (Variables|/Script/UnderForge.PickUpItem|GetHeldPlayer Sword))
                (:then
                  (Default|MULTIDrop _asbp_forge_player))
                (:CastFailed
                  _))
              (Utilities|IsValid Sword
                (:Is%20Valid
                  (Default|GivetoCustomer (Variables|Default|GetCustomerManager) Sword))
                (:Is%20Not%20Valid
                  _))
              (return))))))))

(fn GetCurrentWaveTime
  (bind _wavetimer (Variables|Default|GetWaveTimer))
  (if (Utilities|Time|IsValidTimerHandle _wavetimer)
    (return (+ (Class|KismetSystemLibrary|GetTimerElapsedTimeHandle _wavetimer) (Utilities|Time|GetTimerRemainingTimebyHandle _wavetimer)))
    (else
      (return 0.0))))

(fn GetAvailableWeapons
  (bind (_isvalid _returnvalue) (Class|CommonFunctions|GetGameSingleton))
  (bind _forgegm (CallFunction|GetGamemode))
  (bind (_levelset _valid) (Default|GetCurrentLevel _forgegm))
  (bind _weapons (Variables|/Script/UnderForge.UnderForgeSingleton|GetWeapons _returnvalue))
  (Utilities|IsValid _forgegm
    (:Is%20Valid
      (if _valid
        (LocalVariables|SetAvailableWeapons (.Orders (Utilities|Struct|BreakLevelSet _levelset)))
        (for _array_element (LocalVariables|GetAvailableWeapons) :!label _label
          (if (.ReturnValue (Utilities|Map|Find _weapons _array_element))
            (if (not (.bUsedAsOrder (Utilities|Struct|BreakWeapon (.Value (Utilities|Map|Find _weapons _array_element)))))
              (Utilities|Array|RemoveItem (LocalVariables|GetAvailableWeapons) _array_element))))
        (return (LocalVariables|GetAvailableWeapons))
        (else
          (if _isvalid :!label _label_2
            (bind _keys (Utilities|Map|Keys _weapons))
            (LocalVariables|SetAvailableWeapons _keys)
            (goto _label)))))
    (:Is%20Not%20Valid
      (goto _label_2))))

(fn GainedCurrency
  (params (Gained :type Integer) (NewVal :type Integer))
  (Variables|Default|SetCurrency NewVal)
  (Variables|Default|SetStringCurrency (Utilities|String|ToString(Integer) NewVal))
  (Audio|PlaySound2D "/Game/Sounds/SoundRourke/UI/Coins_Sound.Coins_Sound" 1.0 1.0 0.0 0 0) ; Play Coin/Money sound
)

(fn GetCustomerManager
  (Utilities|IsValid (Variables|Default|GetCustomerManager)
    (:Is%20Valid
      _)
    (:Is%20Not%20Valid
      (bind _returnvalue (Actor|GetActorOfClass "/Game/Blueprints/Customers/CustomerManager.CustomerManager_C"))
      (Variables|Default|SetCustomerManager _returnvalue)))
  (return (Variables|Default|GetCustomerManager)))

(fn OnRepCurrency
  (Variables|Default|SetStringCurrency (Utilities|String|ToString(Integer) (Variables|Default|GetCurrency))))