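; Game mode for a forge level, running a timed day of orders and enemy waves for up to four players.
; BeginPlay syncs local players and controller IDs, then starts a day timed from the level's wave delays in the GameInstance.
; Completed orders pay currency by durability; timer expiry or forge destruction clears enemies and multicasts results through ForgeGameState.
; Restart and next level open the map locally or server-travel online.
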(event EventBeginPlay
  (bind _asforge_game_instance (Utilities|Casting|CastToForgeGameInstance (Game|GetGameInstance)))
  (bind _output_get (Variables|Default|SetGameInstanceRef _asforge_game_instance))
  (if (Variables|/Game/Blueprints/Gameplay/ForgeGameInstance.ForgeGameInstance_C|GetLocal _output_get)
    (CallFunction|AddandRemovePlayers) ; Runs first, gets array of controllers
  )
  (bind _outactors (Actor|GetAllActorsOfClass "/Game/Blueprints/Gameplay/BP_CameraSystem.BP_CameraSystem_C"))
  (bind _output_get_2 (Variables|Default|SetCameraControllerRef (Utilities|Array|Get(acopy) _outactors)))
  (Default|SetControllersView _output_get_2)
  (CallFunction|StartGame)
  (bind _outactors_2 (Actor|GetAllActorsOfClass "/Game/Blueprints/LevelBlueprints/BP_Smeltery.BP_Smeltery_C"))
  (Variables|Default|SetForgeSmelteryRef (Utilities|Array|Get(acopy) _outactors_2)))

(event EventTick
  (params (DeltaSeconds :type Float%20%28single-precision%29)))

(event EventForgeDestroyed
  (CallFunction|EndDay))

(fn ConstructionScript)

(fn AddCurrency
  (params (Gained :type Integer))
  (bind _output_get (Variables|Game|SetCurrency (+ Gained (Variables|Game|GetCurrency))))
  (Default|MULTIGainedCurrency (CallFunction|GetForgeGameState) Gained _output_get)
  (Math|Integer|IncrementInt (Variables|Stats|GetTotalOrdersCompleted)))

(fn NewDay
  (bind _forgegamestate (CallFunction|GetForgeGameState))
  (bind (_levelset _valid) (CallFunction|GetCurrentLevel))
  (Math|Integer|IncrementInt (Variables|DayCycle|GetCurrentDay)
    (:%20%20
      (Variables|/Game/Blueprints/Gameplay/ForgeGameState.ForgeGameState_C|SetCurrentDay (CallFunction|GetForgeGameState) (Variables|DayCycle|GetCurrentDay))
      (bind _leveltime (CallFunction|GetLevelTime))
      (bind _output_get (Variables|DayCycle|SetDayTime _leveltime))
      (bind _returnvalue (Utilities|Time|SetTimerbyFunctionName 0 "EndDay" _output_get))
      (Variables|DayCycle|SetDayTimerHandle _returnvalue)
      (Utilities|IsValid _forgegamestate
        (:Is%20Valid
          (Default|AddBeginningOrders _forgegamestate)
          (if _valid
            (Variables|DayCycle|SetCurrencyNeeded (.CurrencyNeeded (Utilities|Struct|BreakLevelSet _levelset))))
          (Variables|/Game/Blueprints/Gameplay/ForgeGameState.ForgeGameState_C|SetMaxCurrencyNeeded _forgegamestate (Variables|DayCycle|GetCurrencyNeeded)))))))

(fn EndDay
  (Utilities|Time|ClearandInvalidateTimerbyHandle (Variables|DayCycle|GetDayTimerHandle))
  (bind _returnvalue (Actor|GetActorOfClass "/Game/Blueprints/Enemies/EnemyManagerBP.EnemyManagerBP_C"))
  (Utilities|Time|ClearandInvalidateTimerbyHandle (Variables|/Game/Blueprints/Enemies/EnemyManagerBP.EnemyManagerBP_C|GetWaveHandle _returnvalue))
  (Utilities|Time|ClearandInvalidateTimerbyHandle (Variables|/Game/Blueprints/Enemies/EnemyManagerBP.EnemyManagerBP_C|GetEnemySpawningHandle _returnvalue))
  (bind _outactors (Actor|GetAllActorsOfClass "/Game/Blueprints/Enemies/EnemyBase.EnemyBase_C"))
  (for _array_element _outactors
    (Actor|DestroyActor _array_element))
  (CallFunction|CheckDayComplete))

(fn StartGame
  (CallFunction|ResettoStartStas)
  (Game|SetGamePaused false)
  (CallFunction|NewDay)
  (CallFunction|AllPlayersDropActors)
  (CallFunction|RestartPlayers))

(fn RemoveAllPartsItemsandMats
  (bind _outactors (Actor|GetAllActorsOfClass "/Script/UnderForge.ForgePart"))
  (for _array_element _outactors
    (Actor|DestroyActor _array_element))
  (bind _outactors_2 (Actor|GetAllActorsOfClass "/Script/UnderForge.ForgeMat"))
  (for _array_element_2 _outactors_2
    (Actor|DestroyActor _array_element_2))
  (bind _outactors_3 (Actor|GetAllActorsOfClass "/Script/UnderForge.ForgeItem"))
  (for _array_element_3 _outactors_3
    (Actor|DestroyActor _array_element_3))
  (bind _outactors_4 (Actor|GetAllActorsOfClass "/Game/Blueprints/Enemies/EnemyBase.EnemyBase_C"))
  (for _array_element_4 _outactors_4
    (Actor|DestroyActor _array_element_4)))

(fn AllPlayersDropActors
  (for _index (range 0 (- (Variables|Default|GetNumberOfPlayers) 1))
    (bind _asbp_forge_player (Utilities|Casting|CastToBP_ForgePlayer (Game|GetPlayerCharacter _index)))
    (Default|Drop _asbp_forge_player)))

(fn RestartPlayers
  (for _array_element (Variables|Default|GetCurrentPlayerControllers)
    (Utilities|IsValid _array_element
      (:Is%20Valid
        (Class|GameModeBase|RestartPlayer _array_element))))
  (Default|SetControllersView (Variables|Default|GetCameraControllerRef)))

(fn AddandRemovePlayers
  (bind _currentcontrollerid (LocalVariables|GetCurrentControllerID))
  (bind _currentplayercontrollers (Variables|Default|GetCurrentPlayerControllers))
  ;[1 1 1] Spawn extra players
  (for (_array_element _array_index) (Variables|/Game/Blueprints/Gameplay/ForgeGameInstance.ForgeGameInstance_C|GetPlayerState (Variables|Default|GetGameInstanceRef))
    (if _array_element
      (Utilities|IsValid (Game|GetPlayerController _array_index)
        (:Is%20Not%20Valid
          (Class|GameplayStatics|CreatePlayer _array_index)))))
  ;[1 1 1] Get Number of Players
  (for _array_element_2 (Variables|/Game/Blueprints/Gameplay/ForgeGameInstance.ForgeGameInstance_C|GetPlayerState (Variables|Default|GetGameInstanceRef))
    (if _array_element_2
      (Math|Integer|IncrementInt (Variables|Default|GetNumberOfPlayers))))
  ;[1 1 1] Remove Extra Players (Above Count)
  (for _index (range (Variables|Default|GetNumberOfPlayers) 3)
    (Utilities|IsValid (Game|GetPlayerController _index)
      (:Is%20Valid
        ;;[1 1 1] Has to be Twice? thanks unreal
        (Class|GameplayStatics|RemovePlayer (Game|GetPlayerController _index) true)
        (Class|GameplayStatics|RemovePlayer (Game|GetPlayerController _index) true))))
  ;[1 1 1] Set Controller IDs
  (for _index_2 (range 0 3)
    (if (Utilities|Array|Get(acopy) (Variables|/Game/Blueprints/Gameplay/ForgeGameInstance.ForgeGameInstance_C|GetPlayerState (Variables|Default|GetGameInstanceRef)) _index_2)
      (Class|GameplayStatics|SetPlayerControllerID (Game|GetPlayerController _currentcontrollerid) _index_2)
      (Math|Integer|IncrementInt _currentcontrollerid)))
  ;[1 1 1] Add To Controllers Array
  (Utilities|Array|Clear _currentplayercontrollers)
  (for _index_3 (range 0 3)
    (bind _asforge_controller_bp (Utilities|Casting|CastToForgeControllerBP (Game|GetPlayerController _index_3)))
    (Utilities|Array|Add _currentplayercontrollers _asforge_controller_bp)))

(fn ResettoStartStas
  (bind _forgesmelteryref (Variables|Default|GetForgeSmelteryRef))
  (Variables|DayCycle|SetCurrentDay 0)
  (Utilities|IsValid _forgesmelteryref
    (:Is%20Valid
      (Class|Smeltery|RestartHealth _forgesmelteryref))))

(fn CompleteOrder
  (params (OrderID :type Integer) (DurabilityPercentage :type Float%20%28single-precision%29))
  (bind _forgegamestate (CallFunction|GetForgeGameState))
  (Utilities|IsValid _forgegamestate
    (:Is%20Valid
      (Default|CompleteOrder _forgegamestate OrderID))
    (:Is%20Not%20Valid
      _))
  (Math|Integer|IncrementInt (Variables|Stats|GetTotalOrdersCompleted)
    (:%20%20
      (CallFunction|AddCurrency (Math|Float|Truncate (* 10 DurabilityPercentage))))))

(fn GetLatestOrder)

(fn CheckStartScreen
  (bind _intotutwidget (Variables|Default|GetIntoTutWidget))
  (if (Widget|IsVisible _intotutwidget)
    (Widget|SetVisibility _intotutwidget "Hidden")
    (Game|SetGamePaused false)
    (return true)
    (else
      (return false))))

(fn RestartGame
  (bind _returnvalue (Game|GetCurrentLevelName true))
  (LocalVariables|SetCurrentLevel _returnvalue)
  (if (Variables|/Game/Blueprints/Gameplay/ForgeGameInstance.ForgeGameInstance_C|GetLocal (Variables|Default|GetGameInstanceRef))
    (Game|OpenLevel(byName) (Utilities|String|StringToName (LocalVariables|GetCurrentLevel)) :!label _label)
    (else
      (bind _asforge_controller_bp (Utilities|Casting|CastToForgeControllerBP (Game|GetPlayerController 0))
        (:then
          (bind _outactors (Actor|GetAllActorsOfClass "/Game/Blueprints/PlayerBlueprints/ForgeControllerBP.ForgeControllerBP_C"))
          (for _array_element _outactors
            (Default|MULTITryAgain _array_element))
          (Class|NetworkController|ServerTraveltoMap _asforge_controller_bp (LocalVariables|GetCurrentLevel)))
        (:CastFailed
          (goto _label))))))

(fn GetForgeGameState
  (Utilities|IsValid (Variables|Default|GetForgeGameStateRef)
    (:Is%20Valid
      _)
    (:Is%20Not%20Valid
      (bind _asforge_game_state (Utilities|Casting|CastToForgeGameState (Game|GetGameState)))
      (Variables|Default|SetForgeGameStateRef _asforge_game_state)))
  (return (Variables|Default|GetForgeGameStateRef)))

(fn NextLevel
  (bind (_levelset _valid) (CallFunction|GetCurrentLevel))
  (if _valid
    (LocalVariables|SetCurrentNextLevel (.NextLevel (Utilities|Struct|BreakLevelSet _levelset))))
  (if (Variables|/Game/Blueprints/Gameplay/ForgeGameInstance.ForgeGameInstance_C|GetLocal (Variables|Default|GetGameInstanceRef))
    (Game|OpenLevel(byName) (Utilities|String|StringToName (LocalVariables|GetCurrentNextLevel)) :!label _label)
    (else
      (bind _asforge_controller_bp (Utilities|Casting|CastToForgeControllerBP (Game|GetPlayerController 0))
        (:then
          (bind _outactors (Actor|GetAllActorsOfClass "/Game/Blueprints/PlayerBlueprints/ForgeControllerBP.ForgeControllerBP_C"))
          (for _array_element _outactors
            _)
          (Class|NetworkController|ServerTraveltoMap _asforge_controller_bp (LocalVariables|GetCurrentNextLevel)))
        (:CastFailed
          (goto _label))))))

(fn GetLevelTime
  (bind (_levelset _valid) (CallFunction|GetCurrentLevel))
  (bind (_waves _initialdelaytillwaves) (Utilities|Struct|BreakLevelSet _levelset))
  (if _valid
    (LocalVariables|SetCurrentTime _initialdelaytillwaves)
    (for _array_element _waves
      (LocalVariables|SetCurrentTime (+ (LocalVariables|GetCurrentTime) (.delaytillnextwave _array_element))))
    (return (LocalVariables|GetCurrentTime))
    (else
      (return (Variables|DayCycle|GetDayTime)))))

(fn GetCurrentLevel
  (bind _asforge_game_instance (Utilities|Casting|CastToForgeGameInstance (Game|GetGameInstance))
    (:then
      (bind _returnvalue (Game|GetCurrentLevelName true))
      (return (.Value (Utilities|Map|Find (Variables|/Game/Blueprints/Gameplay/ForgeGameInstance.ForgeGameInstance_C|GetLevels _asforge_game_instance) _returnvalue)) (.ReturnValue (Utilities|Map|Find (Variables|/Game/Blueprints/Gameplay/ForgeGameInstance.ForgeGameInstance_C|GetLevels _asforge_game_instance) _returnvalue))))
    (:CastFailed
      (return "" false))))

(fn CheckDayComplete
  (if (not (Utilities|Time|IsValidTimerHandle (Variables|DayCycle|GetDayTimerHandle)))
    (bind _returnvalue (Actor|GetActorOfClass "/Game/Blueprints/Enemies/EnemyManagerBP.EnemyManagerBP_C"))
    (Utilities|IsValid _returnvalue
      (:Is%20Valid
        (if (not (Utilities|Time|IsValidTimerHandle (Variables|/Game/Blueprints/Enemies/EnemyManagerBP.EnemyManagerBP_C|GetWaveHandle _returnvalue)))
          (bind _outactors (Actor|GetAllActorsOfClass "/Game/Blueprints/Enemies/EnemyBase.EnemyBase_C" :!label _label))
          (if (<= (Utilities|Array|Length _outactors) 0)
            (Default|MULTIEndDay (CallFunction|GetForgeGameState) (Variables|Game|GetCurrency) (Variables|DayCycle|GetCurrencyNeeded) (Variables|/Script/UnderForge.Smeltery|GetForgeHealth (Variables|Default|GetForgeSmelteryRef)) :!label _label_2)
            (bind _outactors_2 (Actor|GetAllActorsOfClass "/Game/Blueprints/Enemies/EnemyBase.EnemyBase_C"))
            (for _array_element _outactors_2
              (Actor|DestroyActor _array_element))
            (bind _returnvalue_2 (Actor|GetActorOfClass "/Game/Blueprints/Enemies/EnemyManagerBP.EnemyManagerBP_C"))
            (Utilities|IsValid _returnvalue_2
              (:Is%20Valid
                (Utilities|Time|ClearandInvalidateTimerbyHandle (Variables|/Game/Blueprints/Enemies/EnemyManagerBP.EnemyManagerBP_C|GetWaveHandle _returnvalue_2))
                (Utilities|Time|ClearandInvalidateTimerbyHandle (Variables|/Game/Blueprints/Enemies/EnemyManagerBP.EnemyManagerBP_C|GetEnemySpawningHandle _returnvalue_2)))
              (:Is%20Not%20Valid
                _))
            (Utilities|Time|ClearandInvalidateTimerbyHandle (Variables|/Game/Blueprints/Gameplay/ForgeGameState.ForgeGameState_C|GetOrdersHandle (CallFunction|GetForgeGameState)))
            (elif (and (<= (Variables|/Game/Blueprints/Enemies/EnemyBase.EnemyBase_C|GetHealth (Utilities|Array|Get(acopy) _outactors)) 0) (<= (Utilities|Array|Length _outactors) 1))
              (goto _label_2)))))
      (:Is%20Not%20Valid
        (goto _label)))))