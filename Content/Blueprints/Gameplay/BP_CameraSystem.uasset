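; BP_CameraSystem is an actor that serves as a shared camera view target for players in the Forge level.
; On BeginPlay, non-authority instances switch the local player controller's view to this actor.
; SetControllersView lazily caches the GM_ForgeLevel game mode, then points every valid controller in its CurrentPlayerControllers list at this actor.
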(event EventBeginPlay
  (Networking|SwitchHasAuthority
    (:Remote
      (Game|Player|SetViewTargetwithBlend (Game|GetPlayerController 0) self 0.0 "VTBlend_Linear" 0.0 false))))

(event Collision|EventActorBeginOverlap
  (params (OtherActor :type Actor%20Object%20Reference)))

(event EventTick
  (params (DeltaSeconds :type Float%20%28single-precision%29)))

(fn ConstructionScript)

(fn SetControllersView
  (Utilities|IsValid (Variables|Default|GetForgeGamemode)
    (:Is%20Valid
      _)
    (:Is%20Not%20Valid
      (bind _asgm_forge_level (Utilities|Casting|CastToGM_ForgeLevel (Game|GetGameMode)))
      (Variables|Default|SetForgeGamemode _asgm_forge_level)))
  (for _array_element (Variables|/Game/Blueprints/Gameplay/GM_ForgeLevel.GM_ForgeLevel_C|GetCurrentPlayerControllers (Variables|Default|GetForgeGamemode))
    (Utilities|IsValid _array_element
      (:Is%20Valid
        (Game|Player|SetViewTargetwithBlend _array_element self 0.0 "VTBlend_Linear" 0.0 false)))))