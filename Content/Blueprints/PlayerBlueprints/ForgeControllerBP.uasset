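; Player controller for the forge game, managing each player's order HUD, pause input and end-of-round screen.
; On BeginPlay, controller ID 0 switches to the shared camera, creates the HUD and plays background sound; remote instances also request current orders.
; Order updates go to a lazily created HUD, while server events relay order and wave-timer syncs through ForgeGameState.
; Round end shows a stats screen with UI-only input, which try-again clears.
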(event Custom|SERVER_GetOrders
  (bind _asforge_game_state (Utilities|Casting|CastToForgeGameState (Game|GetGameState)))
  (Default|SSendOutOrders _asforge_game_state))

(event Custom|SERVER_UpdateWaveTimer
  (bind _asforge_game_state (Utilities|Casting|CastToForgeGameState (Game|GetGameState)))
  (Default|MULTIStartWaveTimer _asforge_game_state (Utilities|Time|GetTimerRemainingTimebyHandle (Variables|/Game/Blueprints/Mechanics/ForgeGameState.ForgeGameState_C|GetWaveTimer _asforge_game_state))))

(event Custom|MULTI_TryAgain
  (Utilities|IsValid (Variables|Default|GetEnd%20Screen)
    (:Is%20Valid
      (Widget|RemovefromParent (Variables|Default|GetEnd%20Screen)))
    (:Is%20Not%20Valid
      _))
  (Variables|Default|SetEnd%20Screen 0)
  (Variables|Default|SetbShowMouseCursor true)
  (Input|SetInputModeGameOnly self))

(event EventBeginPlay
  (if (== (Class|GameplayStatics|GetPlayerControllerID self) 0)
    (bind _returnvalue (Actor|GetActorOfClass "/Game/Blueprints/Mechanics/BP_CameraSystem.BP_CameraSystem_C"))
    (Utilities|IsValid _returnvalue
      (:Is%20Valid
        (Game|Player|SetViewTargetwithBlend _returnvalue 0.0 "VTBlend_Linear" 0.0 false))
      (:Is%20Not%20Valid
        _))
    (Utilities|IsValid (CallFunction|GetForgeHUD)
      (:Is%20Valid
        _)
      (:Is%20Not%20Valid
        (Development|PrintString "Couldn't get/Create Hud" true true "(R=1.000000,G=0.006452,B=0.000000,A=1.000000)" 5.0)))
    (Audio|PlaySound2D (Variables|Default|GetBackgroundSound) 0.3 1.0 0.0 0 0)
    (Networking|SwitchHasAuthority
      (:Remote
        (CallFunction|SERVERGetOrders)))))

(event EventTick
  (params (DeltaSeconds :type Float%20%28single-precision%29)))

(event EventEndRound
  (params (Currency :type Integer) (CurrencyNeeded :type Integer))
  (CallFunction|EndRoundScreen Currency CurrencyNeeded 0.0))

(event Input|ActionEvents|InputActionMenu
  (params (Key :type Key%20Structure :default "None"))
  (:Pressed
    (bind _asgm_forge_level (Utilities|Casting|CastToGM_ForgeLevel (Game|GetGameMode)))
    (bind _hasstartscreen (Default|CheckStartScreen _asgm_forge_level))
    (if (not _hasstartscreen)
      (Default|TogglePauseGame _asgm_forge_level))))

(fn ConstructionScript)

(fn PrintOutID
  (Development|PrintString (Utilities|String|Append "PLAYER WITH ID " (Utilities|String|ToString(Integer) (Class|GameplayStatics|GetPlayerControllerID self))) true true "(R=0.000000,G=0.660000,B=1.000000,A=1.000000)" 1e+01))

(fn NewOrder
  (params (Weapon :type EWeapon%20Enum :default "W_NONE") (ID :type Integer%20%28by%20ref%29))
  (bind _hudref (CallFunction|GetForgeHUD))
  (Utilities|IsValid _hudref
    (:Is%20Valid
      (Default|AddOrder _hudref Weapon ID))))

(fn CompleteOrder
  (params (OrderID :type Integer))
  (bind _hudref (CallFunction|GetForgeHUD))
  (Utilities|IsValid _hudref
    (:Is%20Valid
      (Default|OrderComplete _hudref OrderID))))

(fn GetForgeHUD
  (Utilities|IsValid (Variables|Default|GetHUDRef)
    (:Is%20Valid
      _)
    (:Is%20Not%20Valid
      (bind _returnvalue (UserInterface|CreateWidget "/Game/UI/W_HUD.W_HUD_C" self))
      (bind _output_get (Variables|Default|SetHUDRef _returnvalue))
      (UserInterface|Viewport|AddtoViewport _output_get 0)))
  (return (Variables|Default|GetHUDRef)))

(fn EndRoundScreen
  (params (Currency :type Integer) (CurrencyNeeded :type Integer) (ForgeHealth :type Float%20%28single-precision%29))
  (bind _returnvalue (UserInterface|CreateWidget "/Game/UI/Screens/W_EndScreen.W_EndScreen_C" self))
  (UserInterface|Viewport|AddtoViewport _returnvalue 0)
  (bind _output_get (Variables|Default|SetEnd%20Screen _returnvalue))
  (Default|SetEndStats _output_get (Utilities|Array|Length (Variables|/Script/Engine.GameStateBase|GetPlayerArray (Game|GetGameState))) 0 0 0 Currency CurrencyNeeded (* ForgeHealth 1e+02))
  (Variables|Default|SetbShowMouseCursor true)
  (Input|SetInputModeUIOnly self (Variables|/Game/UI/Screens/W_EndScreen.W_EndScreen_C|GetTryAgainBtn (Variables|Default|GetEnd%20Screen)) "DoNotLock"))