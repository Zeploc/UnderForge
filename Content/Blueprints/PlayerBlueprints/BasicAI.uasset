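; BasicAI is a character Blueprint with a forward obstacle-detection helper and no active behavior.
; RayCastCheck sweeps an oriented box from just below the capsule's center along its forward vector for a given distance and trace channel, with optional debug drawing.
; It exits through Hit with the struck actor or through Missed.
; A move-to-player call and a sphere trace are left unconnected, and nothing here calls RayCastCheck.
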(fn ConstructionScript)