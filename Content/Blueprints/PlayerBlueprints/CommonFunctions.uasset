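; Shared player helper that resolves a crafted weapon type from an array of weapon parts.
; GetWeaponFromParts loops over the parts, keeping the last handle and last blade it identifies.
; Nested selects map that pair to one of eight enum values, splitting on Kris versus any other handle, then on four blade types.
; No invalid case exists, so unmatched parts fall through to a default weapon.
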(fn GetWeaponfromParts
  (params (Parts :type Array%20of%20ESwordPart%20Enums :default "PT_NONE"))
  (for _array_element Parts
    (if (Class|CommonFunctions|IsHandle _array_element)
      (LocalVariables|SetHandle _array_element)
      (elif (Class|CommonFunctions|IsBlade _array_element)
        (LocalVariables|SetBlade _array_element))))
  (return (select (Utilities|Enum|Equal(Enum) (LocalVariables|GetHandle) "PT_KRISHANDLE") (select (or (Utilities|Enum|Equal(Enum) (LocalVariables|GetBlade) "PT_IRONKRISBLADE") (Utilities|Enum|Equal(Enum) (LocalVariables|GetBlade) "PT_IRONBROADSWORDBLADE")) (select (Utilities|Enum|Equal(Enum) (LocalVariables|GetBlade) "PT_IRONBROADSWORDBLADE") "NewEnumerator2" "NewEnumerator0") (select (Utilities|Enum|Equal(Enum) (LocalVariables|GetBlade) "PT_STEELBROADSWORDBLADE") "NewEnumerator3" "NewEnumerator1")) (select (or (Utilities|Enum|Equal(Enum) (LocalVariables|GetBlade) "PT_IRONKRISBLADE") (Utilities|Enum|Equal(Enum) (LocalVariables|GetBlade) "PT_IRONBROADSWORDBLADE")) (select (Utilities|Enum|Equal(Enum) (LocalVariables|GetBlade) "PT_IRONBROADSWORDBLADE") "NewEnumerator6" "NewEnumerator4") (select (Utilities|Enum|Equal(Enum) (LocalVariables|GetBlade) "PT_STEELBROADSWORDBLADE") "NewEnumerator7" "NewEnumerator5")))))