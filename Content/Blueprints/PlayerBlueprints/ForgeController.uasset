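; ForgeController is a player controller for the forge level, with pause input and debug tools for checking local multiplayer controllers.
; The Menu input toggles pause through the GM_ForgeLevel game mode, and BeginPlay prints the controller's ID.
; SecondaryInteract loops over the first four player indices, prints which exist, and calls PrintOutID on each ForgeController to print its ID.
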(event EventBeginPlay
  (bind _returnvalue (Class|GameplayStatics|GetPlayerControllerID self))
  (Development|PrintString (Utilities|String|Append "Creating Controller " (Utilities|String|ToString(Integer) _returnvalue)) true true "(R=0.000000,G=0.660000,B=1.000000,A=1.000000)" 1e+01))

(event EventTick
  (params (DeltaSeconds :type Float%20%28single-precision%29)))

(event Input|ActionEvents|InputActionMenu
  (params (Key :type Key%20Structure))
  (:Pressed
    (bind _asgm_forge_level (Utilities|Casting|CastToGM_ForgeLevel (Game|GetGameMode)))
    (Default|TogglePauseGame _asgm_forge_level)))

(event Input|ActionEvents|InputActionSecondaryInteract
  (params (Key :type Key%20Structure))
  (:Pressed
    (for _index (range 0 3)
      (Utilities|IsValid (Game|GetPlayerController _index)
        (:Is%20Valid
          (Development|PrintString (Utilities|String|Append "Player " (Utilities|String|ToString(Integer) _index) " Exists") true true "(R=0.000000,G=0.660000,B=1.000000,A=1.000000)" 1e+01)
          (bind _asforge_controller (Utilities|Casting|CastToForgeController (Game|GetPlayerController _index)))
          (CallFunction|PrintOutID _asforge_controller))))))

(fn ConstructionScript)

(fn PrintOutID
  (bind _returnvalue (Class|GameplayStatics|GetPlayerControllerID self))
  (Development|PrintString (Utilities|String|Append "PLAYER WITH ID " (Utilities|String|ToString(Integer) _returnvalue)) true true "(R=0.000000,G=0.660000,B=1.000000,A=1.000000)" 1e+01))