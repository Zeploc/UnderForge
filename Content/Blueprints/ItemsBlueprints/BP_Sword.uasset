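; BP_Sword is a sword item with limited durability that starts at its maximum on BeginPlay.
; SwordDurability decrements it and, at zero, calls WeaponBreak on the player, plays a break sound and destroys the sword.
; SetHasBeenLaunched flags the sword as launched and starts a timer to EnableCanLaunch, which also sets that flag true rather than clearing it.
; A node enabling mesh physics on launch is disconnected.
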(event EventBeginPlay
  (Variables|Default|SetDurability (Variables|Default|GetMaxDurability)))

(event Collision|EventActorBeginOverlap
  (params (OtherActor :type Actor%20Object%20Reference)))

(event EventTick
  (params (DeltaSeconds :type Float%20%28single-precision%29)))

(fn ConstructionScript)

(fn SetHasBeenLaunched
  (Variables|Default|SetHasBeenLaunched true)
  (Utilities|Time|SetTimerbyFunctionName 0 "EnableCanLaunch" (Variables|Default|GetResetTime)))

(fn EnableCanLaunch
  (Variables|Default|SetHasBeenLaunched true))

(fn SwordDurability
  (params (Player :type BP%20Forge%20Player%20Object%20Reference))
  (Math|Integer|DecrementInt (Variables|Default|GetDurability)
    (:%20%20
      (if (<= (Variables|Default|GetDurability) 0)
        (Default|WeaponBreak Player)
        (Audio|PlaySound2D "/Game/Sounds/SoundRourke/UI/FlagBreak_Cue.FlagBreak_Cue" 1.0 1.0 0.0 0 0)
        (Actor|DestroyActor)))))