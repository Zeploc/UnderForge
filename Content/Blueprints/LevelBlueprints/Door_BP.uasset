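; Door actor that swings open for EnemyBase actors and closes once none remain in its trigger box.
; Box overlap events track enemies in EnemiesInTrigger and set the goal yaw to open on entry, or closed when the last one leaves.
; Every Tick, RotateDoor turns the DoorRotatePoint pivot toward that goal using constant-rate RInterpToConstant at DoorSpeed.
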(event OnComponentBeginOverlap(Box)
  (params (OverlappedComponent :type Primitive%20Component%20Object%20Reference) (OtherActor :type Actor%20Object%20Reference) (OtherComp :type Primitive%20Component%20Object%20Reference) (OtherBodyIndex :type Integer) (bFromSweep :type Boolean) (SweepResult :type Hit%20Result%20Structure%20%28by%20ref%29))
  (bind _asenemy_base (Utilities|Casting|CastToEnemyBase OtherActor))
  (Utilities|Array|Add (Variables|Default|GetEnemiesInTrigger) _asenemy_base)
  (Variables|Default|SetGoalRotation 1.2e+02))

(event OnComponentEndOverlap(Box)
  (params (OverlappedComponent :type Primitive%20Component%20Object%20Reference) (OtherActor :type Actor%20Object%20Reference) (OtherComp :type Primitive%20Component%20Object%20Reference) (OtherBodyIndex :type Integer))
  (bind _asenemy_base (Utilities|Casting|CastToEnemyBase OtherActor))
  (Utilities|Array|RemoveItem (Variables|Default|GetEnemiesInTrigger) _asenemy_base)
  (if (<= (Utilities|Array|Length (Variables|Default|GetEnemiesInTrigger)) 0)
    (Variables|Default|SetGoalRotation 0.0)))

(event EventBeginPlay)

(event Collision|EventActorBeginOverlap
  (params (OtherActor :type Actor%20Object%20Reference)))

(event EventTick
  (params (DeltaSeconds :type Float%20%28single-precision%29))
  (CallFunction|RotateDoor DeltaSeconds))

(fn ConstructionScript)

(fn RotateDoor
  (params (Delta :type Float%20%28single-precision%29))
  (bind _doorrotatepoint (Variables|Default|GetDoorRotatePoint))
  (Transformation|SetRelativeRotation _doorrotatepoint (Class|KismetMathLibrary|RInterptoConstant (Variables|/Script/Engine.SceneComponent|GetRelativeRotation _doorrotatepoint) (Math|Rotator|MakeRotator 0.0 0.0 (Variables|Default|GetGoalRotation)) Delta (Variables|Default|GetDoorSpeed)) false false))