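; BP_CombineBench is a bench actor that holds weapon parts (blades and handles) and a current item.
; Tick shows the Display component while PotentiallyInteracting is set, using a timer to clear that flag after a short timeout.
; ThrowOutParts destroys the current item, then maps each stored part type to its Blueprint class, spawns it at the Display, throws it away and empties the list.
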(event Custom|ThrowOutParts
  (bind _currentparts (Variables|Default|GetCurrentParts))
  (Utilities|IsValid (Variables|Default|GetCurrentItem)
    (:Is%20Valid
      (Actor|DestroyActor (Variables|Default|GetCurrentItem))
      (Variables|Default|SetCurrentItem 0))
    (:Is%20Not%20Valid
      _))
  (for _array_element _currentparts
    (bind _returnvalue (Game|SpawnActorfromClass (Utilities|Select :Index _array_element :PT_NONE 0 :PT_IRONKRISBLADE "/Game/Blueprints/ItemsBlueprints/BP_IronKrisBladePart.BP_IronKrisBladePart_C" :PT_IRONBROADSWORDBLADE "/Game/Blueprints/ItemsBlueprints/BP_IronBroadswordBladePart.BP_IronBroadswordBladePart_C" :PT_STEELKRISBLADE "/Game/Blueprints/ItemsBlueprints/BP_SteelKrisBladePart.BP_SteelKrisBladePart_C" :PT_STEELBROADSWORDBLADE "/Game/Blueprints/ItemsBlueprints/BP_SteelBroadswordBladePart.BP_SteelBroadswordBladePart_C" :PT_KRISHANDLE "/Game/Blueprints/ItemsBlueprints/BP_KrisHandlePart.BP_KrisHandlePart_C" :PT_BROADSWORDHANDLE "/Game/Blueprints/ItemsBlueprints/BP_BroadswordHandlePart.BP_BroadswordHandlePart_C") (Transformation|GetWorldTransform (Variables|Default|GetDisplay)) "Undefined" 0 0))
    (Class|ForgeStation|ThrowAway _returnvalue))
  (Utilities|Array|Clear _currentparts))

(event EventBeginPlay
  (Variables|Default|SetTimer 0.0))

(event Collision|EventActorBeginOverlap
  (params (OtherActor :type Actor%20Object%20Reference)))

(event EventTick
  (params (DeltaSeconds :type Float%20%28single-precision%29))
  (if (>= (Variables|Default|GetTimer) 1.5)
    (Variables|Default|SetPotentiallyInteracting false)
    (Variables|Default|SetTimer 0.0))
  (if (Variables|Default|GetPotentiallyInteracting)
    (Variables|Default|SetTimer (+ DeltaSeconds (Variables|Default|GetTimer)))
    (if (not (Variables|/Script/Engine.SceneComponent|GetbVisible (Variables|Default|GetDisplay)))
      (Rendering|SetVisibility (Variables|Default|GetDisplay) true false))
    (elif (Variables|/Script/Engine.SceneComponent|GetbVisible (Variables|Default|GetDisplay))
      (Rendering|SetVisibility (Variables|Default|GetDisplay) false false))))

(fn ConstructionScript)