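; Smeltery crafting station that registers tin and iron ore-to-ingot recipes and links itself to its timer and health widgets.
; Resource interface events update the timer's ForgeDisplay widget, while material processing only prints a debug message.
; Tick toggles fire, smoke and sound during the minigame, orients the timer toward the camera, and computes melt or overcook progress from the remaining time's sign.
; Interaction highlight uses custom depth stencil, with its flag cleared every frame.
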(event EventBeginPlay
  (bind _self self)
  (bind _asforge_display (Utilities|Casting|CastToForgeDisplay (UserInterface|GetUserWidgetObject (Variables|Components|GetSmeltery%20Time))))
  (Variables|Default|SetForgeDisplayWidget _asforge_display)
  (Default|SetOwningStation _asforge_display _self)
  (bind _asforge_health (Utilities|Casting|CastToForgeHealth (UserInterface|GetUserWidgetObject (Variables|Components|GetHealth))))
  (Default|SetSmelteryReference _asforge_health _self)
  (CallFunction|OrientateWidget (Variables|Components|GetSmeltery%20Time))
  (Utilities|Map|Add (Variables|Default|GetIngotRecipies) "R_TININGOT" (Utilities|Struct|MakeIngotRecipe 1 (Utilities|Array|MakeArray "R_TINORE") 5.0))
  (Utilities|Map|Add (Variables|Default|GetIngotRecipies) "R_IRONINGOT" (Utilities|Struct|MakeIngotRecipe 1 (Utilities|Array|MakeArray "R_IRONORE") 5.0)))

(event Collision|EventActorBeginOverlap
  (params (OtherActor :type Actor%20Object%20Reference)))

(event EventBIonNewResource
  (params (_Resource :type EResource%20Enum :default "R_WOOD"))
  (Default|AddResource (Variables|Default|GetForgeDisplayWidget) _Resource))

(event EventTick
  (params (DeltaSeconds :type Float%20%28single-precision%29))
  (CallFunction|BurningEffect)
  (CallFunction|OrientateWidget (Variables|Components|GetSmeltery%20Time))
  (CallFunction|SetCurrentTimeRemaining)
  (Rendering|SetCustomDepthStencilValue (Variables|Default|GetStationMesh) (Math|Conversions|ToInteger(Boolean) (Variables|Default|GetPotentiallyInteracting)))
  (Class|ForgeStation|SetPotentiallyInteracting false))

(event EventBIonRemoveResource
  (params (_Resource :type EResource%20Enum :default "R_WOOD"))
  (Default|RemoveResource (Variables|Default|GetForgeDisplayWidget) _Resource))

(event EventBIonSetPotentiallyInteracting)

(event EventBIonProcessMatItem
  (params (material :type Forge%20Mat%20Object%20Reference))
  (Development|PrintString (Utilities|String|Append "Process Mat " (Utilities|String|EnumtoString (Variables|/Script/UnderForge.ForgeMat|GetResourceType material))) true false "(R=0.952433,G=1.000000,B=0.884944,A=1.000000)" 5.0))

(fn ConstructionScript)

(fn OrientateWidget
  (params (Widget :type Widget%20Component%20Object%20Reference))
  (bind _returnvalue (Transformation|GetWorldLocation Widget))
  (bind _returnvalue_2 (Game|GetPlayerCameraManager 0))
  (bind _returnvalue_3 (Camera|GetCameraLocation _returnvalue_2))
  (bind _returnvalue_4 (Math|Rotator|FindLookatRotation _returnvalue _returnvalue_3))
  (Utilities|IsValid Widget
    (:Is%20Valid
      (Transformation|SetWorldRotation Widget (Math|Rotator|MakeRotator 0.0 (.pitch _returnvalue_4) (+ (* (.roll _returnvalue_4) -1.0) 9e+01)) false false))))

(fn BurningEffect
  (bind _flamesound (Variables|Components|GetFlameSound))
  (bind _particlesystem (Variables|Components|GetParticleSystem))
  (bind _smoke (Variables|Components|GetSmoke))
  (bind _burning (Variables|Components|GetBurning))
  (bind _returnvalue (Components|Activation|IsActive _burning))
  (if (<= (Variables|Default|GetCurrentRemainingTime) 0.0)
    (if _returnvalue :!label _label
      (Components|Activation|Deactivate _burning)
      (Components|Activation|Deactivate _particlesystem)
      (Components|Activation|Deactivate _smoke))
    (if (Audio|Components|Audio|IsPlaying (Variables|Components|GetFlameSound))
      (Audio|Components|Audio|Stop (Variables|Components|GetFlameSound)))
    (elif (Variables|Default|GetbSmeltingMinigamePlaying)
      (if _returnvalue
        _
        (else
          (Components|Activation|Activate _burning true)
          (Components|Activation|Activate _particlesystem true)
          (Components|Activation|Activate _smoke true)))
      (if (not (Audio|Components|Audio|IsPlaying _flamesound))
        (Audio|Components|Audio|Play _flamesound 0.0))
      (else
        (goto _label)))))

(fn SetCurrentTimeRemaining
  (bind _currentrecipesmeltingtimeneeded (Variables|Default|GetCurrentRecipeSmeltingTimeNeeded))
  (bind _currentremainingtime (Variables|Default|GetCurrentRemainingTime))
  (if (> _currentremainingtime 0.0)
    (Variables|Default|SetMeltingPercentage (- 1.0 (/ _currentremainingtime _currentrecipesmeltingtimeneeded)))
    (elif (< _currentremainingtime 0.0)
      (Variables|Default|SetMeltingPercentage (- 1.0 (/ (* _currentremainingtime -1.0) (- (Variables|Default|GetSmeltingTimeKABOOM) _currentrecipesmeltingtimeneeded))))
      (else
        (Variables|Default|SetMeltingPercentage 0.0)))))

(fn OnSetPotentiallyInteract
  (params (Potentially :type Boolean))
  (if (not Potentially)
    (Utilities|Time|SetTimerbyFunctionName 0 "TryHideInteract" 1.0)))

(fn TryHideInteract
  (if (Variables|Default|GetPotentiallyInteracting)
    (Utilities|Time|SetTimerbyFunctionName 0 "TryHideInteract" 1.0)))

(fn DebugPrint
  (for (_array_element _array_index) (Variables|Default|GetCurrentlyProcessing)
    (Development|PrintString (Utilities|String|Append (Utilities|String|ToString(Integer) _array_index) ": " (Utilities|String|EnumtoString _array_element)) true false "(R=1.000000,G=0.703719,B=0.753715,A=1.000000)" 0.001))
  (bind _keys (Utilities|Map|Keys (Variables|Default|GetIngotRecipies)))
  (for _array_element_2 _keys
    (Development|PrintString (Utilities|String|Append (Utilities|String|EnumtoString _array_element_2) " Uses " (Utilities|String|EnumtoString (Utilities|Array|Get(acopy) (.Resources (Utilities|Struct|BreakIngotRecipe (.Value (Utilities|Map|Find (Variables|Default|GetIngotRecipies) _array_element_2))))))) true false "(R=1.000000,G=0.703719,B=0.753715,A=1.000000)" 0.001)))